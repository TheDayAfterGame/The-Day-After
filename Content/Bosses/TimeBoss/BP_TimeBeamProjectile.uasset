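; Time Boss beam projectile that extends from its spawn point along a direction and explodes on impact or on timeout.
; Tick stretches and thickens the actor between lerped endpoints while sphere-tracing its length, ignoring owner and player.
; CreateExplosion spawns BP_TimeExplosion, shakes the camera and damages overlapping BP_ThirdPersonCharacter actors in a width-scaled radius.
; The beam then locks its length and width, collapses its tail toward the far end and destroys itself.
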(event EventTick
  (params (DeltaSeconds :type Float%20%28single-precision%29))
  (bind _returnvalue (Transformation|GetActorScale3D))
  (bind (_x _y _z) (Math|Vector|BreakVector _returnvalue))
  (bind _output_get (Variables|Default|SetTimeAlive (+ (Variables|Default|GetTimeAlive) (* DeltaSeconds (Variables|Default|GetSpeed) 0.6))))
  (if (Variables|Default|GetRetreating)
    (CallFunction|SetPosition (.Start (Utilities|LerpStartEnd (- 1.0 (/ _output_get 0.4)) true)) (.End (Utilities|LerpStartEnd (- 1.0 (/ _output_get 0.4)) true)))
    (if (<= (- 1.0 (/ _output_get 0.4)) 0.0)
      (Actor|DestroyActor))
    (elif (Variables|Default|GetTraveling)
      (CallFunction|SetPosition (.Start (Utilities|LerpStartEnd (Math|Float|Power (/ _output_get 0.8) 1.3) false)) (.End (Utilities|LerpStartEnd (Math|Float|Power (/ _output_get 0.8) 1.3) false)))
      (if (>= (Variables|Default|GetTimeAlive) 1.0)
        (Variables|Default|SetTraveling false :!label _label)
        (CallFunction|CreateExplosion (Math|Vector|SelectVector (.End (Utilities|LerpStartEnd (Math|Float|Power (/ _output_get 0.8) 1.3) false)) (.Location (Collision|BreakHitResult (stale _outhit))) (>= (Variables|Default|GetTimeAlive) 1.0)))
        (Variables|Default|SetMaxDistance (* _z 1e+02))
        (Variables|Default|SetTimeAlive 0.0)
        (Variables|Default|SetRetreating true)
        (else
          (bind (_outhit _returnvalue_2) (Collision|SphereTraceForObjects (.Start (Utilities|LerpStartEnd (Math|Float|Power (/ _output_get 0.8) 1.3) false)) (.End (Utilities|LerpStartEnd (Math|Float|Power (/ _output_get 0.8) 1.3) false)) (* _x 1e+02) (|ArrayofObjectTypes_2) false (Utilities|Array|MakeArray (Components|GetOwner) (Game|GetPlayerCharacter 0)) "None"))
          (if _returnvalue_2
            (goto _label)))))))

(fn ConstructionScript
  (Variables|Default|SetStartLocation (Transformation|GetWorldLocation (Variables|Default|GetDefaultSceneRoot))))

(fn CreateExplosion
  (params (Position :type Vector))
  (LocalVariables|SetRadius (* (.X (Math|Vector|BreakVector (Transformation|GetActorScale3D))) 1.8e+02))
  (Game|SpawnActorfromClass "/Game/Bosses/TimeBoss/BP_TimeExplosion.BP_TimeExplosion_C" (Math|Conversions|ToTransform(Vector) Position) "AlwaysSpawn" 0 0)
  (Camera|PlayWorldCameraShake "/Game/Enemies/AI/BP_HitShake_Boss.BP_HitShake_Boss_C" Position 0.0 (* (LocalVariables|GetRadius) 1.5) 0.0)
  (bind _outactors (Collision|SphereOverlapActors Position (LocalVariables|GetRadius) (|ArrayofObjectTypes_2_2) "/Game/ThirdPerson/Blueprints/BP_ThirdPersonCharacter.BP_ThirdPersonCharacter_C"))
  (for _array_element _outactors
    (Game|Damage|ApplyDamage _array_element 3.0 0 (Components|GetOwner))
    (Development|PrintString (Utilities|GetDisplayName _array_element))))

(fn SetPosition
  (params (Start :type Vector) (End :type Vector))
  (bind _returnvalue (Math|Vector|Distance(Vector) Start End))
  (bind _returnvalue_2 (Transformation|GetActorScale3D))
  (bind _retreating (Variables|Default|GetRetreating))
  (bind _x (Math|Vector|BreakVector _returnvalue_2))
  (bind _returnvalue_3 (/ _returnvalue 2.5e+03))
  (bind _returnvalue_4 (+ _returnvalue_3 0.4))
  (bind _returnvalue_5 (Math|Float|Power _returnvalue_4 0.3))
  (bind _returnvalue_6 (select _retreating _x _returnvalue_5))
  (Transformation|SetActorLocation (/ (+ Start End) "2.000000,2.000000,2.000000") false true)
  (Transformation|SetActorScale3D (Math|Vector|MakeVector _returnvalue_6 _returnvalue_6 (/ _returnvalue 1e+02))))