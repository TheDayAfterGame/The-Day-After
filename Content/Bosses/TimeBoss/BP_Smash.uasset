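; BP_Smash is the Time Boss's smash attack, caching its owning BP_TimeBoss on BeginPlay.
; Use plays the smash montage on the boss at the given speed and prints the returned duration; the target input is unused.
; CreateExplosion is a separate function that spawns a damaging BP_Smash_Explosion at a given location, with no caller in this file.
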(event EventBeginPlay
  (|CallParentFunction)
  (bind _asbp_time_boss (Utilities|Casting|CastToBP_TimeBoss (Components|GetOwner)))
  (Variables|Default|SetCharacter _asbp_time_boss))

(event EventTick
  (params (DeltaSeconds :type Float%20%28single-precision%29))
  (|CallParentFunction DeltaSeconds) ; This node is disabled and will not be called.\nDrag off pins to build functionality.
)

(fn Use
  (params (Target :type Vector :default "0, 0, 0") (Speed :type Float%20%28double-precision%29))
  (bind _returnvalue (Animation|PlayAnimMontage (Variables|Default|GetCharacter) "/Game/Bosses/TimeBoss/Animations/Smash_Montage.Smash_Montage" Speed "None"))
  (Development|PrintString (Utilities|String|ToString(Float) _returnvalue)))

(fn CreateExplosion
  (params (Location :type Vector))
  (Game|SpawnActorfromClass "/Game/Bosses/TimeBoss/BP_Smash_Explosion.BP_Smash_Explosion_C" (Math|Conversions|ToTransform(Vector) Location) "AlwaysSpawn" 0 5e+01 0))