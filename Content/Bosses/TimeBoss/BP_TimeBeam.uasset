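; BP_TimeBeam is a Time Boss attack that charges up with particles, then fires a BP_TimeBeamProjectile toward a target.
; Start stores the target and activates the charge particles.
; Use spawns the projectile at StartActor's location at zero initial scale, facing the target, passes it a normalized direction, speed and the boss-side owner, then deactivates the particles.
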(event EventBeginPlay
  (|CallParentFunction) ; This node is disabled and will not be called.\nDrag off pins to build functionality.
)

(event EventTick
  (params (DeltaSeconds :type Float%20%28single-precision%29))
  (|CallParentFunction DeltaSeconds) ; This node is disabled and will not be called.\nDrag off pins to build functionality.
)

(fn Use
  (params (Target :type Vector :default "0, 0, 0") (Speed :type Float%20%28double-precision%29))
  (bind _output_get (LocalVariables|SetStart (Transformation|GetWorldLocation (Variables|Default|GetStartActor))))
  (Game|SpawnActorfromClass "/Game/Bosses/TimeBoss/BP_TimeBeamProjectile.BP_TimeBeamProjectile_C" (Math|Transform|MakeTransform _output_get (Math|Rotator|FindLookatRotation _output_get Target) "0.000000,0.000000,0.000000") "AlwaysSpawn" (Components|GetOwner) (Math|Vector|Normalize (- Target _output_get)) Speed 0)
  (Components|Activation|Deactivate (Variables|Default|GetChargeParticles)))

(fn Start
  (params (Target :type Vector :default "0, 0, 0") (Speed :type Float%20%28double-precision%29))
  (Variables|Default|SetTarget Target)
  (Components|Activation|Activate (Variables|Default|GetChargeParticles) false))