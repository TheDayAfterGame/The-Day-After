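; Time Boss enemy with tiered health phases, where each tier changes max health and speeds up attack timings and cooldowns.
; Attack picks a weighted random beam, stalactite or smash component that is off cooldown and unlocked, then runs Start, Use and End with delays.
; Lethal damage below the last tier flags a phase change, which refills health at the next Attack.
; BeginPlay sets Tier 2 then advances, so the fight opens at tier 3.
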(event EventBeginPlay
  (|CallParentFunction)
  (Variables|Default|SetTier 2)
  (CallFunction|AdvancetoNextTier))

(event Collision|EventActorBeginOverlap
  (params (OtherActor :type Actor%20Object%20Reference)))

(event EventTick
  (params (DeltaSeconds :type Float%20%28single-precision%29))
  (bind _bossattacks (Variables|Default|GetBossAttacks))
  (bind _keys (Utilities|Map|Keys _bossattacks))
  (for _array_element _keys
    (Utilities|Map|Add _bossattacks _array_element (- (.Value (Utilities|Map|Find _bossattacks _array_element)) (* DeltaSeconds (.Speed (CallFunction|GetSpeed 0.0)))))))

(event EventAttack
  (bind _returnvalue (Game|Player|GetPlayerPawn 0))
  (bind _returnvalue_2 (Transformation|GetActorLocation _returnvalue))
  (if (Variables|Default|GetisDead)
    (Default|CallOnAttackEnd :!label _label)
    (elif (Variables|Default|GetShouldAdvanceToNextTier)
      (CallFunction|AdvancetoNextTier)
      (Utilities|FlowControl|Delay 5.0)
      (goto _label)
      (else
        (bind _attack (CallFunction|GetNextAttack))
        (Utilities|IsValid (.Attack (Utilities|Struct|BreakBossAttack _attack))
          (:Is%20Valid
            (Development|PrintString "Start")
            (Default|Start (.Attack (Utilities|Struct|BreakBossAttack _attack)) _returnvalue_2 (.Speed (CallFunction|GetSpeed (Variables|/Game/Bosses/TimeBoss/BP_BossAttack.BP_BossAttack_C|GetStartup (.Attack (Utilities|Struct|BreakBossAttack _attack))))))
            (Utilities|FlowControl|Delay (.New%20Duration (CallFunction|GetSpeed (Variables|/Game/Bosses/TimeBoss/BP_BossAttack.BP_BossAttack_C|GetStartup (.Attack (Utilities|Struct|BreakBossAttack _attack))))))
            (Development|PrintString "Use")
            (Default|Use (.Attack (Utilities|Struct|BreakBossAttack _attack)) _returnvalue_2 (.Speed (CallFunction|GetSpeed (Variables|/Game/Bosses/TimeBoss/BP_BossAttack.BP_BossAttack_C|GetDuration (.Attack (Utilities|Struct|BreakBossAttack _attack))))))
            (Utilities|FlowControl|Delay (.New%20Duration (CallFunction|GetSpeed (Variables|/Game/Bosses/TimeBoss/BP_BossAttack.BP_BossAttack_C|GetDuration (.Attack (Utilities|Struct|BreakBossAttack _attack))))))
            (Development|PrintString "End")
            (Default|End (.Attack (Utilities|Struct|BreakBossAttack _attack)) (.Speed (CallFunction|GetSpeed (Variables|/Game/Bosses/TimeBoss/BP_BossAttack.BP_BossAttack_C|GetEndlag (.Attack (Utilities|Struct|BreakBossAttack _attack))))))
            (Utilities|FlowControl|Delay (.New%20Duration (CallFunction|GetSpeed (Variables|/Game/Bosses/TimeBoss/BP_BossAttack.BP_BossAttack_C|GetEndlag (.Attack (Utilities|Struct|BreakBossAttack _attack))))))
            (Development|PrintString "Done")
            (Utilities|Map|Add (Variables|Default|GetBossAttacks) _attack (.Cooldown (Utilities|Struct|BreakBossAttack _attack)))
            (Default|CallOnAttackEnd))
          (:Is%20Not%20Valid
            (goto _label)))))))

(event EventRemoveSword)

(event EventSheathSword)

(event EventSpawnSword)

(event EventAnyDamage
  (params (Damage :type Float%20%28single-precision%29) (DamageType :type Damage%20Type%20Object%20Reference) (InstigatedBy :type Controller%20Object%20Reference) (DamageCauser :type Actor%20Object%20Reference))
  (bind _bp_healthbar (Variables|Default|GetBP_HealthBar))
  (bind _health (Variables|/Game/RangedEnemy/Blueprints/BP_HealthBar.BP_HealthBar_C|GetHealth _bp_healthbar))
  (if (and (<= _health Damage) (< (Variables|Default|GetTier) 4))
    (if (Variables|Default|GetShouldAdvanceToNextTier)
      (CallFunction|OnDamage (- _health 0.01) DamageCauser)
      (else
        (Variables|Default|SetShouldAdvanceToNextTier true)))
    (else
      (CallFunction|OnDamage Damage DamageCauser))))

(fn ConstructionScript
  (bind _bossattacks (Variables|Default|GetBossAttacks))
  (bind _bp_timebeam (Variables|Default|GetBP_TimeBeam))
  (Variables|/Game/Bosses/TimeBoss/BP_TimeBeam.BP_TimeBeam_C|SetStartActor _bp_timebeam (Variables|Default|GetOrb))
  (Variables|/Game/Bosses/TimeBoss/BP_TimeBeam.BP_TimeBeam_C|SetChargeParticles _bp_timebeam (Variables|Default|GetChargeParticles))
  (|CallParentFunction)
  (Utilities|Map|Clear _bossattacks)
  (Utilities|FlowControl|Sequence
    (:then_0
      (Utilities|Map|Add _bossattacks (Utilities|Struct|MakeBossAttack 3.0 3 4.0 (Variables|Default|GetBP_TimeBeam)) 0.0))
    (:then_1
      (Utilities|Map|Add _bossattacks (Utilities|Struct|MakeBossAttack 2e+01 2 2.0 (Variables|Default|GetBP_Stalactites)) 0.0))
    (:then_2
      (Utilities|Map|Add _bossattacks (Utilities|Struct|MakeBossAttack 0.0 1 3.0 (Variables|Default|GetBP_Smash)) 0.0))))

(fn GetNextAttack
  (bind _bossattacks (Variables|Default|GetBossAttacks))
  (bind _keys (Utilities|Map|Keys _bossattacks))
  (for _array_element _keys
    (if (and (<= (.Value (Utilities|Map|Find _bossattacks _array_element)) 0.0) (>= (Variables|Default|GetTier) (.Tier (Utilities|Struct|BreakBossAttack _array_element))))
      (Utilities|Array|Add (LocalVariables|GetAvailableAttacks) _array_element)
      (LocalVariables|SetTotalWeight (+ (LocalVariables|GetTotalWeight) (.Weight (Utilities|Struct|BreakBossAttack _array_element))))))
  (LocalVariables|SetSelectedWeight (Math|Random|RandomFloatinRange 0.0 (LocalVariables|GetTotalWeight)))
  (for _array_element_2 (LocalVariables|GetAvailableAttacks)
    (if (<= (LocalVariables|GetSelectedWeight) (.Weight (Utilities|Struct|BreakBossAttack _array_element_2)))
      (return _array_element_2)
      (else
        (LocalVariables|SetSelectedWeight (- (LocalVariables|GetSelectedWeight) (.Weight (Utilities|Struct|BreakBossAttack _array_element_2)))))))
  (return ""))

(fn GetSpeed
  (params (Duration :type Float%20%28double-precision%29))
  (bind _tier (Variables|Default|GetTier))
  (bind _returnvalue (Utilities|Select :Index _tier :Option%200 1.0 :Option%201 1.0 :Option%202 1.25 :Option%203 1.5 :Option%204 2.0))
  (return (/ Duration _returnvalue) _returnvalue))

(fn AdvancetoNextTier
  (bind _bp_healthbar (Variables|Default|GetBP_HealthBar))
  (bind _output_get (Variables|Default|SetTier (+ (Variables|Default|GetTier) 1)))
  (Variables|Default|SetShouldAdvanceToNextTier false)
  (if (<= _output_get 4)
    (bind _output_get_2 (Variables|/Game/RangedEnemy/Blueprints/BP_HealthBar.BP_HealthBar_C|SetMaxHealth _bp_healthbar (Utilities|Select :Index _output_get :Option%200 0.0 :Option%201 4e+03 :Option%202 3e+03 :Option%203 2e+03 :Option%204 1.5e+03)))
    (Variables|/Game/RangedEnemy/Blueprints/BP_HealthBar.BP_HealthBar_C|SetHealth _bp_healthbar _output_get_2)
    (Default|UpdateHealthBar _bp_healthbar)
    (return false)
    (else
      (return true))))

(fn CreateSmashExplosion
  (Default|CreateExplosion (Variables|Default|GetBP_Smash) (Transformation|GetWorldLocation (Variables|Character|GetMesh))))