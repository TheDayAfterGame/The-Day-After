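; BP_Smash_Explosion is the time boss's smash explosion actor, a one-shot area hit.
; On BeginPlay it plays a boss hit camera shake around itself and runs a pawn overlap query using its Cylinder component.
; Each overlapped third-person player character takes the configured Damage, with a debug print.
; The actor destroys itself when its particle system finishes.
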(event OnSystemFinished(Particles)
  (params (PSystem :type Niagara%20Component%20Object%20Reference))
  (Actor|DestroyActor))

(event EventBeginPlay
  (bind _cylinder (Variables|Default|GetCylinder))
  (Camera|PlayWorldCameraShake "/Game/Enemies/AI/BP_HitShake_Boss.BP_HitShake_Boss_C" (Transformation|GetActorLocation) 0.0 7.5e+02 0.0)
  (bind _outactors (Collision|ComponentOverlapActors _cylinder (Transformation|GetWorldTransform _cylinder) (Utilities|Array|MakeArray "ObjectTypeQuery3") 0))
  (for _array_element _outactors
    (bind _asbp_third_person_character (Utilities|Casting|CastToBP_ThirdPersonCharacter _array_element))
    (Game|Damage|ApplyDamage _asbp_third_person_character (Variables|Default|GetDamage) 0 0)
    (Development|PrintString "smash hit player")))

(event Collision|EventActorBeginOverlap
  (params (OtherActor :type Actor%20Object%20Reference)))

(event EventTick
  (params (DeltaSeconds :type Float%20%28single-precision%29)))

(fn ConstructionScript)