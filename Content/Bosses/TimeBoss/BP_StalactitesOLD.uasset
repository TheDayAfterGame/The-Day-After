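; Time boss stalactite hazard that fills the roof with BP_Stalactite actors and drops them one at a time.
; Spawn count scales with roof area and density, with random positions and slight tilts within the roof bounds.
; The tick interval spreads drops across AttackDuration, each tick enabling physics on the next valid stalactite's cone.
; Once the array empties, it pauses, regenerates, then resumes dropping after a second delay.
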(event EventBeginPlay
  (CallFunction|Regenerate)
  (Class|ActorComponent|SetComponentTickInterval (/ (Variables|Default|GetAttackDuration) (CallFunction|GetNumStalactites))))

(event EventTick
  (params (DeltaSeconds :type Float%20%28single-precision%29))
  (bind _stalactites (Variables|Default|GetStalactites))
  (bind _output (Utilities|Array|Get(acopy) _stalactites))
  (if (Variables|Default|GetShouldDrop)
    (if (Utilities|Array|IsNotEmpty _stalactites) :!label _label
      (Utilities|IsValid _output
        (:Is%20Valid
          (Physics|SetSimulatePhysics (Variables|/Game/Bosses/TimeBoss/BP_Stalactite.BP_Stalactite_C|GetCone _output) true)
          (Utilities|Array|RemoveIndex _stalactites))
        (:Is%20Not%20Valid
          (Utilities|Array|RemoveIndex _stalactites)
          (goto _label)))
      (else
        (Variables|Default|SetShouldDrop false)
        (Utilities|FlowControl|Delay 5.0)
        (CallFunction|Regenerate)
        (Utilities|FlowControl|Delay 3.0)
        (Variables|Default|SetShouldDrop true)))))

(fn GenerateStalactites
  (params (Count :type Integer))
  (for _index (range 1 Count)
    (bind _returnvalue (Game|SpawnActorfromClass "/Game/Bosses/TimeBoss/BP_Stalactite.BP_Stalactite_C" (CallFunction|GetRandomSpawnLocation) "AdjustIfPossibleButAlwaysSpawn" 0 0))
    (Utilities|Array|Add (Variables|Default|GetStalactites) _returnvalue)))

(fn GetRandomSpawnLocation
  (bind _returnvalue (Math|Random|RandomFloatinRange -5.0 5.0))
  (bind _returnvalue_2 (Math|Float|MakeLiteralFloat -1.0))
  (bind _roof (Variables|Default|GetRoof))
  (bind (_origin _boxextent) (Collision|GetActorBounds _roof false false))
  (bind (_x _y) (Math|Vector|BreakVector _boxextent))
  (return (Math|Transform|MakeTransform (+ _origin (Math|Vector|MakeVector (Math|Random|RandomFloatinRange (* _x _returnvalue_2) _x) (Math|Random|RandomFloatinRange (* _y _returnvalue_2) _y) 0.0)) (Math|Rotator|MakeRotator _returnvalue _returnvalue 0.0))))

(fn Regenerate
  (CallFunction|GenerateStalactites (CallFunction|GetNumStalactites)))

(fn GetNumStalactites
  (bind _roof (Variables|Default|GetRoof))
  (bind _boxextent (Collision|GetActorBounds _roof false false))
  (bind (_x _y) (Math|Vector|BreakVector _boxextent))
  (return (Math|Float|Floor (* (Variables|Default|GetStalactiteDensity) 4.0 _x _y 0.0001))))