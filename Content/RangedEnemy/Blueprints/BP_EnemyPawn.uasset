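; Ranged enemy pawn that shoots at a player it sees and takes damage through a health bar component.
; PawnSensing sets the target, then Tick line-traces to it each frame, turning the capsule by yaw and firing on a cooldown until sight is lost.
; FireBullet spawns projectiles just outside the capsule along the aim direction; a hitscan alternative exists but never runs.
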(event OnSeePawn(PawnSensing)
  (params (Pawn :type Pawn%20Object%20Reference))
  (bind _asbp_third_person_character (Utilities|Casting|CastToBP_ThirdPersonCharacter Pawn))
  (if (!= _asbp_third_person_character (Variables|Default|GetSpottedPlayer))
    (Variables|Default|SetSpottedPlayer _asbp_third_person_character)
    (Variables|Default|SetShooting true)
    (Variables|Default|SetShotCooldown 0.5)))

(event EventBeginPlay
  (Default|UpdateHealthBar (Variables|Default|GetBP_HealthBar)))

(event Collision|EventActorBeginOverlap
  (params (OtherActor :type Actor%20Object%20Reference)))

(event EventTick
  (params (DeltaSeconds :type Float%20%28single-precision%29))
  (bind _capsule (Variables|Default|GetCapsule))
  (bind _returnvalue (Transformation|GetSocketLocation _capsule "Center"))
  (bind _output_get (Variables|Default|SetShotCooldown (- (Variables|Default|GetShotCooldown) DeltaSeconds)))
  (if (Variables|Default|GetShooting)
    (bind (_outhit _returnvalue_2) (Collision|LineTraceForObjects _returnvalue (Transformation|GetWorldLocation (Variables|/Script/Engine.Character|GetCapsuleComponent (Variables|Default|GetSpottedPlayer))) (|ArrayofObjectTypes) false 0 "None"))
    (if _returnvalue_2
      (bind _asbp_third_person_character (Utilities|Casting|CastToBP_ThirdPersonCharacter (.HitActor (Collision|BreakHitResult _outhit)))
        (:then
          (CallFunction|FacePlayer _returnvalue (.Location (Collision|BreakHitResult _outhit)) DeltaSeconds)
          (if (<= _output_get 0.0)
            (CallFunction|FireBullet (- (.Location (Collision|BreakHitResult _outhit)) _returnvalue))
            (Variables|Default|SetShotCooldown 0.5)))
        (:CastFailed
          (Variables|Default|SetShooting false :!label _label)
          (Variables|Default|SetSpottedPlayer _asbp_third_person_character)))
      (else
        (goto _label)))))

(event Game|Damage|EventAnyDamage
  (params (Damage :type Float%20%28single-precision%29) (DamageType :type Damage%20Type%20Object%20Reference) (InstigatedBy :type Controller%20Object%20Reference) (DamageCauser :type Actor%20Object%20Reference))
  (Default|TakeDamage (Variables|Default|GetBP_HealthBar) Damage))

(fn ConstructionScript)

(fn FireBullet
  (params (Direction :type Vector))
  (bind _returnvalue (Math|Vector|Normalize Direction))
  (bind _capsule (Variables|Default|GetCapsule))
  (bind _capsule_2 (Variables|Default|GetCapsule))
  (bind _returnvalue_2 (Math|Vector|Distance2D(Vector) _returnvalue "0, 0, 0"))
  (bind _returnvalue_3 (Transformation|GetSocketLocation _capsule_2 "Center"))
  (bind _capsuleradius (Variables|/Script/Engine.CapsuleComponent|GetCapsuleRadius _capsule))
  (bind _returnvalue_4 (+ 17.0 _capsuleradius))
  (bind _returnvalue_5 (/ _returnvalue_4 _returnvalue_2))
  (bind _returnvalue_6 (* _returnvalue _returnvalue_5))
  (bind _returnvalue_7 (+ _returnvalue_6 _returnvalue_3))
  (Game|SpawnActorfromClass "/Game/RangedEnemy/Blueprints/BP_EnemyProjectile.BP_EnemyProjectile_C" (Math|Transform|MakeTransform _returnvalue_7 (Math|Rotator|FindLookatRotation _returnvalue_3 _returnvalue_7)) "AlwaysSpawn" 0 0))

(fn FacePlayer
  (params (Start :type Vector%20%28by%20ref%29) (Target :type Vector) (DeltaTime :type Float%20%28double-precision%29))
  (Transformation|SetWorldRotation (Variables|Default|GetCapsule) (Math|Interpolation|RInterpTo (Transformation|GetWorldRotation (Variables|Default|GetCapsule)) (Math|Rotator|MakeRotator 0.0 0.0 (.Yaw (Math|Rotator|BreakRotator (Math|Rotator|FindLookatRotation Start Target)))) DeltaTime 1e+01) false false)
  (Class|PrimitiveComponent|SetPhysicsAngularVelocityinDegrees (Variables|Default|GetCapsule) "0, 0, 0" false "None"))