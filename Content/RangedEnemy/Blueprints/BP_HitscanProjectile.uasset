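; BP_HitscanProjectile is an actor that represents a ranged enemy's hitscan shot as a segment between a rifle and an end point.
; UpdateTransform places the root midway between the Rifle mesh's Ammo socket and EndLocation, with look-at rotation toward the end.
; It stretches Z scale by the distance divided by 100.
; The event graph is empty, so the update relies on an external call.
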(event EventBeginPlay)

(event Collision|EventActorBeginOverlap
  (params (OtherActor :type Actor%20Object%20Reference)))

(event EventTick
  (params (DeltaSeconds :type Float%20%28single-precision%29)))

(fn ConstructionScript)

(fn UpdateTransform
  (bind _rifle (Variables|Default|GetRifle))
  (bind _endlocation (Variables|Default|GetEndLocation))
  (bind _skeletalmesh (Variables|/Game/RangedEnemy/Blueprints/BP_Rifle_Hitscan.BP_Rifle_Hitscan_C|GetSkeletalMesh _rifle))
  (bind _returnvalue (Transformation|GetSocketLocation _skeletalmesh "Ammo"))
  (Transformation|SetWorldTransform (Variables|Default|GetDefaultSceneRoot) (Math|Transform|MakeTransform (/ (+ _returnvalue _endlocation) "2.000000,2.000000,2.000000") (Math|Rotator|FindLookatRotation _returnvalue _endlocation) (Math|Vector|MakeVector 1.0 1.0 (/ (Math|Vector|Distance(Vector) _returnvalue _endlocation) 1e+02))) false false))