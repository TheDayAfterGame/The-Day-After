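; Ranged enemy character that spots the third-person player through pawn sensing and tracks it as a target.
; Blackboard keys mirror range, target and shooting state; a line trace each tick records the target's angle or clears both target and shooting when sight is lost.
; Damage feeds the health bar.
; Helpers turn the capsule and fire rifle projectiles, but the Tick logic calling them is disconnected.
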(event OnSeePawn(PawnSensing)
  (params (Pawn :type Pawn%20Object%20Reference))
  (bind _asbp_third_person_character (Utilities|Casting|CastToBP_ThirdPersonCharacter Pawn))
  (if (!= _asbp_third_person_character (Variables|Default|GetSpottedPlayer))
    (CallFunction|SetTarget _asbp_third_person_character)
    (CallFunction|SetShooting true)
    (Variables|Default|SetShotCooldown 0.5)))

(event OnTargetPerceptionUpdated(AIPerception)
  (params (Actor :type Actor%20Object%20Reference) (Stimulus :type AI%20Stimulus%20Structure))
  (Development|PrintString "Seen target"))

(event EventBeginPlay
  (Default|UpdateHealthBar (Variables|Default|GetBP_HealthBar))
  (AI|Components|Blackboard|SetValueasFloat (AI|GetBlackboard 0) (Utilities|Name|MakeLiteralName "Range") (Variables|Default|GetRange))
  (CallFunction|SetShooting false))

(event EventTick
  (params (DeltaSeconds :type Float%20%28single-precision%29))
  (bind _output_get (Variables|Default|SetShotCooldown (- (Variables|Default|GetShotCooldown) DeltaSeconds)))
  (if (Variables|Default|GetShooting)
    (bind (_outhit _returnvalue) (Collision|LineTraceForObjects (Transformation|GetSocketLocation (Variables|Collision|GetCapsuleComponent) "Center") (Transformation|GetWorldLocation (Variables|/Script/Engine.Character|GetCapsuleComponent (Variables|Default|GetSpottedPlayer))) (|ArrayofObjectTypes_2) false 0 "None"))
    (if _returnvalue
      (Utilities|Casting|CastToBP_ThirdPersonCharacter (.HitActor (Collision|BreakHitResult _outhit))
        (:then
          (Variables|Default|SetPreviousTargetAngle (CallFunction|GetTargetAngle)))
        (:CastFailed
          (CallFunction|SetShooting false :!label _label)
          (CallFunction|SetTarget)))
      (else
        (goto _label)))))

(event Game|Damage|EventAnyDamage
  (params (Damage :type Float%20%28single-precision%29) (DamageType :type Damage%20Type%20Object%20Reference) (InstigatedBy :type Controller%20Object%20Reference) (DamageCauser :type Actor%20Object%20Reference))
  (Default|TakeDamage (Variables|Default|GetBP_HealthBar) Damage))

(fn ConstructionScript)

(fn FireBullet
  (bind _returnvalue (Utilities|GetTargetVector))
  (bind _rifle (Variables|Default|GetRifle))
  (bind _capsulecomponent (Variables|Collision|GetCapsuleComponent))
  (bind _returnvalue_2 (Transformation|GetSocketLocation _rifle "Muzzle"))
  (bind _capsuleradius (Variables|/Script/Engine.CapsuleComponent|GetCapsuleRadius _capsulecomponent))
  (bind _returnvalue_3 (* _returnvalue _capsuleradius))
  (bind _returnvalue_4 (+ _returnvalue_3 _returnvalue_2))
  (Game|SpawnActorfromClass "/Game/RangedEnemy/Blueprints/BP_EnemyProjectile.BP_EnemyProjectile_C" (Math|Transform|MakeTransform _returnvalue_4 (Math|Rotator|FindLookatRotation _returnvalue_2 _returnvalue_4)) "AlwaysSpawn" 0 0)
  (Variables|Default|SetShotCooldown 0.5))

(fn FacePlayer
  (params (Start :type Vector%20%28by%20ref%29) (Target :type Vector) (DeltaTime :type Float%20%28double-precision%29))
  (bind _capsulecomponent (Variables|Collision|GetCapsuleComponent))
  (Transformation|SetWorldRotation _capsulecomponent (Math|Interpolation|RInterpTo (Transformation|GetWorldRotation (Variables|Collision|GetCapsuleComponent)) (Math|Rotator|MakeRotator 0.0 0.0 (.Yaw (Math|Rotator|BreakRotator (Math|Rotator|FindLookatRotation Start Target)))) DeltaTime 1e+01) false false)
  (Class|PrimitiveComponent|SetPhysicsAngularVelocityinDegrees _capsulecomponent "0, 0, 0" false "None"))

(fn SetShooting
  (params (Shooting :type Boolean))
  (bind _output_get (Variables|Default|SetShooting Shooting))
  (AI|Components|Blackboard|SetValueasBool (AI|GetBlackboard 0) (Utilities|Name|MakeLiteralName "Shooting") _output_get))

(fn SetTarget
  (params (Target :type BP%20Third%20Person%20Character%20Object%20Reference))
  (AI|Components|Blackboard|SetValueasObject (AI|GetBlackboard 0) (Utilities|Name|MakeLiteralName "Target") Target)
  (Variables|Default|SetSpottedPlayer Target))

(fn GetTargetAngle
  (bind _spottedplayer (Variables|Default|GetSpottedPlayer))
  (Utilities|IsValid _spottedplayer
    (:Is%20Valid
      (return (Math|Rotator|FindLookatRotation (Transformation|GetWorldLocation (Variables|Collision|GetCapsuleComponent)) (Transformation|GetActorLocation _spottedplayer))))))