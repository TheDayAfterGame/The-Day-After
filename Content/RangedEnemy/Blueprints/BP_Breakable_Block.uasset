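; BP_Breakable_Block is a damageable block actor whose durability depends on its size.
; The construction script multiplies the health bar component's MaxHealth by the square root of the static mesh's world-scale volume, so larger blocks get more health.
; BeginPlay refreshes the BPHealthBar, and any damage received is forwarded to its TakeDamage, leaving health handling to that component.
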(event EventBeginPlay
  (Default|UpdateHealthBar (Variables|Default|GetBP_HealthBar)))

(event Collision|EventActorBeginOverlap
  (params (OtherActor :type Actor%20Object%20Reference)))

(event EventTick
  (params (DeltaSeconds :type Float%20%28single-precision%29)))

(event Game|Damage|EventAnyDamage
  (params (Damage :type Float%20%28single-precision%29) (DamageType :type Damage%20Type%20Object%20Reference) (InstigatedBy :type Controller%20Object%20Reference) (DamageCauser :type Actor%20Object%20Reference))
  (Default|TakeDamage (Variables|Default|GetBP_HealthBar) Damage))

(fn ConstructionScript
  (bind _bp_healthbar (Variables|Default|GetBP_HealthBar))
  (bind _staticmeshcomponent (Variables|Debug|GetStaticMeshComponent))
  (bind _returnvalue (Transformation|GetWorldScale _staticmeshcomponent))
  (bind (_x _y _z) (Math|Vector|BreakVector _returnvalue))
  (Variables|/Game/RangedEnemy/Blueprints/BP_HealthBar.BP_HealthBar_C|SetMaxHealth _bp_healthbar (* (Math|Float|Sqrt (* _x _y _z)) (Variables|/Game/RangedEnemy/Blueprints/BP_HealthBar.BP_HealthBar_C|GetMaxHealth _bp_healthbar))))