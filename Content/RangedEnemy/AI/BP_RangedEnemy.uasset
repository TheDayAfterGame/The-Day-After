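; Rifle-armed enemy character that fires projectiles as its attack, overriding the parent's sword events with empty ones.
; Attack waits briefly, calls FireBullet, plays the shoot montage and signals attack end.
; FireBullet spawns BP_EnemyProjectile near the muzzle along GetTargetVector, whose logic is unconnected, gated by a cooldown that Tick counts down.
; While alive, Tick also stores the look-at rotation toward the blackboard's AttackTarget as PreviousTargetAngle.
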(event EventBeginPlay
  (|CallParentFunction) ; This node is disabled and will not be called.\nDrag off pins to build functionality.
)

(event Collision|EventActorBeginOverlap
  (params (OtherActor :type Actor%20Object%20Reference)))

(event EventTick
  (params (DeltaSeconds :type Float%20%28single-precision%29))
  (Variables|Default|SetShotCooldown (- (Variables|Default|GetShotCooldown) DeltaSeconds))
  (if (not (Variables|Default|GetisDead))
    (Utilities|Casting|CastToActor (AI|Components|Blackboard|GetValueasObject (AI|GetBlackboard 0) (Utilities|Name|MakeLiteralName "AttackTarget")))
    (Variables|Default|SetPreviousTargetAngle (CallFunction|GetTargetAngle))))

(event EventAttack
  (if (not (Variables|Default|GetisDead))
    (Utilities|FlowControl|Delay 0.2)
    (CallFunction|FireBullet)
    (Animation|PlayAnimMontage "/Game/RangedEnemy/AI/Animation/REnemy_Shoot_Montage.REnemy_Shoot_Montage" 1.0 "None")
    (Default|CallOnAttackEnd)))

(event EventRemoveSword)

(event EventSheathSword)

(event EventSpawnSword)

(fn ConstructionScript
  (|CallParentFunction))

(fn FireBullet
  (bind _returnvalue (Utilities|GetTargetVector))
  (bind _rifle (Variables|Default|GetRifle))
  (bind _capsulecomponent (Variables|Default|GetCapsuleComponent))
  (bind _returnvalue_2 (Transformation|GetSocketLocation _rifle "Muzzle"))
  (bind _capsuleradius (Variables|/Script/Engine.CapsuleComponent|GetCapsuleRadius _capsulecomponent))
  (bind _returnvalue_3 (* _returnvalue _capsuleradius))
  (bind _returnvalue_4 (+ _returnvalue_3 _returnvalue_2))
  (if (<= (Variables|Default|GetShotCooldown) 0.0)
    (Game|SpawnActorfromClass "/Game/RangedEnemy/Blueprints/BP_EnemyProjectile.BP_EnemyProjectile_C" (Math|Transform|MakeTransform _returnvalue_4 (Math|Rotator|FindLookatRotation _returnvalue_2 _returnvalue_4)) "AlwaysSpawn" 0 0)
    (Variables|Default|SetShotCooldown 0.5)))

(fn GetTargetAngle
  (bind _asactor (Utilities|Casting|CastToActor (AI|Components|Blackboard|GetValueasObject (AI|GetBlackboard 0) (Utilities|Name|MakeLiteralName "AttackTarget"))))
  (return (Math|Rotator|FindLookatRotation (Transformation|GetWorldLocation (Variables|Default|GetCapsuleComponent)) (Transformation|GetActorLocation _asactor))))