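; Inventory function library for saving and loading items and looking up item, consumable and module data.
; The three getters use the enum's string as a data table row name.
; SaveGame's entry is unwired; its orphaned nodes would write class and quantity arrays to a SaveGameGogglesnort slot.
; LoadGame reads those arrays and finds the third-person character, but its inventory rebuild loop is disconnected.
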(fn SaveGame
  (params (SaveName :type String)))

(fn LoadGame
  (params (SaveGame :type String))
  (Development|PrintString 0 "loading game")
  (bind _returnvalue (SaveGame|LoadGamefromSlot SaveGame))
  (Utilities|IsValid _returnvalue
    (:Is%20Valid
      (bind _assave_game_gogglesnort (Utilities|Casting|CastToSaveGameGogglesnort _returnvalue)
        (:then
          (LocalVariables|SetItemClasses (Variables|/Game/Saving/SaveGameGogglesnort.SaveGameGogglesnort_C|GetItemsArray _assave_game_gogglesnort))
          (LocalVariables|SetItemQuantities (Variables|/Game/Saving/SaveGameGogglesnort.SaveGameGogglesnort_C|GetItemsQuantity _assave_game_gogglesnort))
          (bind _returnvalue_2 (Actor|GetActorOfClass 0 "/Game/ThirdPerson/Blueprints/BP_ThirdPersonCharacter.BP_ThirdPersonCharacter_C")))
        (:CastFailed
          (Development|PrintString 0 "AAAAAH ERROR WHEN LOADING GAME!!" :!label _label))))
    (:Is%20Not%20Valid
      (goto _label))))

(fn GetDatafromEnum
  (params (Item%20type :type ItemName%20Enum :default "NewEnumerator0") (__WorldContext :type Object%20Object%20Reference))
  (bind _returnvalue (Utilities|GetDataTableRow "/Game/Inventory/ItemData/ItemData.ItemData" (Utilities|String|StringToName (Utilities|String|EnumtoString Item%20type)))
    (:then
      (return _returnvalue))
    (:RowNotFound
      (return ""))))

(fn GetCDatafromEnum
  (params (Item%20type :type ItemName%20Enum :default "NewEnumerator0") (__WorldContext :type Object%20Object%20Reference))
  (bind _returnvalue (Utilities|GetDataTableRow "/Game/Inventory/ItemData/ConsumablesDataTable.ConsumablesDataTable" (Utilities|String|StringToName (Utilities|String|EnumtoString Item%20type)))
    (:then
      (return _returnvalue))
    (:RowNotFound
      (return ""))))

(fn GetMDatafromEnum
  (params (Item%20type :type ItemName%20Enum :default "NewEnumerator0") (__WorldContext :type Object%20Object%20Reference))
  (bind _returnvalue (Utilities|GetDataTableRow "/Game/Inventory/ItemData/ModuleDataTable.ModuleDataTable" (Utilities|String|StringToName (Utilities|String|EnumtoString Item%20type)))
    (:then
      (return _returnvalue))
    (:RowNotFound
      (return ""))))