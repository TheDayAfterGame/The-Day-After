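; ConsumableObject is a world representation of a consumable inventory item, shown as a slowly spinning mesh.
; On BeginPlay it looks up data by its ItemName through GetDataFromEnum, assigns that mesh and multiplies the mesh's relative scale by the item's scale.
; Tick yaws the root by DeltaSeconds plus one degree each frame, so spin speed depends on frame rate.
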(event EventBeginPlay
  (bind _staticmesh (Variables|Default|GetStaticMesh))
  (bind _item_name (Variables|Default|GetItem%20Name))
  (bind _returnvalue (Transformation|GetRelativeTransform _staticmesh))
  (bind _out_row (CallFunction|GetDatafromEnum _item_name))
  (bind (_itemenum _itemtype _name _description _mesh _icon _itemscale) (Utilities|Struct|BreakItemKeys _out_row))
  (Components|StaticMesh|SetStaticMesh _staticmesh _mesh)
  (Transformation|SetRelativeTransform _staticmesh (Math|Transform|MakeTransform (.location _returnvalue) (.rotation _returnvalue) (* (.scale _returnvalue) _itemscale)) false false))

(event EventTick
  (params (DeltaSeconds :type Float%20%28single-precision%29))
  (Transformation|AddLocalRotation (Variables|Default|GetDefaultSceneRoot) (Math|Rotator|MakeRotator 0.0 0.0 (+ DeltaSeconds 1.0)) false false))

(fn ConstructionScript)