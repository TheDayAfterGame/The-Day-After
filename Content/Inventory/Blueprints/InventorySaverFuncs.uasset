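; Function library that saves and loads the player's inventory through an InventorySaver object in the "inventory" save slot.
; SaveInventory reads the inventory screens directly, storing modules with an installed flag, consumables with quantities, and the scrap total.
; LoadInventory rebuilds the screens by re-adding each consumable unit, adding scrap and toggling installed modules.
; Loading does nothing when no valid save exists, and does not clear the screens first.
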(fn LoadInventory
  (params (Inventory :type Main%20Inventory%20Object%20Reference))
  (bind _consumablesscreen (Variables|/Game/Inventory/Blueprints/UI2/MainInventory.MainInventory_C|GetConsumablesScreen Inventory))
  (bind _modulesscreen (Variables|/Game/Inventory/Blueprints/UI2/MainInventory.MainInventory_C|GetModulesScreen Inventory))
  (bind _returnvalue (SaveGame|LoadGamefromSlot "inventory"))
  (bind _asinventory_saver (Utilities|Casting|CastToInventorySaver _returnvalue))
  (bind _keys (Utilities|Map|Keys (Variables|/Game/Inventory/Blueprints/InventorySaver.InventorySaver_C|GetConsumables _asinventory_saver)))
  (for _array_element _keys
    (for _index (range 1 (.Value (Utilities|Map|Find (Variables|/Game/Inventory/Blueprints/InventorySaver.InventorySaver_C|GetConsumables _asinventory_saver) _array_element)))
      (Default|Add _consumablesscreen _array_element)))
  (Default|AddScrap _consumablesscreen (Variables|/Game/Inventory/Blueprints/InventorySaver.InventorySaver_C|GetScrap _asinventory_saver))
  (bind _keys_2 (Utilities|Map|Keys (Variables|/Game/Inventory/Blueprints/InventorySaver.InventorySaver_C|GetModules _asinventory_saver)))
  (for _array_element_2 _keys_2
    (Default|Add _modulesscreen _array_element_2)
    (if (.Value (Utilities|Map|Find (Variables|/Game/Inventory/Blueprints/InventorySaver.InventorySaver_C|GetModules _asinventory_saver) _array_element_2))
      (Default|ToggleInstallationItem _modulesscreen _array_element_2))))

(fn SaveInventory
  (params (Inventory :type Main%20Inventory%20Object%20Reference))
  (bind _modulesscreen (Variables|/Game/Inventory/Blueprints/UI2/MainInventory.MainInventory_C|GetModulesScreen Inventory))
  (bind _consumablesscreen (Variables|/Game/Inventory/Blueprints/UI2/MainInventory.MainInventory_C|GetConsumablesScreen Inventory))
  (bind _returnvalue (Game|ConstructObjectfromClass Inventory "/Game/Inventory/Blueprints/InventorySaver.InventorySaver_C"))
  (bind _output_get (Variables|/Game/Inventory/Blueprints/InventorySaver.InventorySaver_C|SetModules _returnvalue (Utilities|Map|MakeMap "NewEnumerator7" false)))
  (Utilities|Map|Clear _output_get)
  (for _array_element (Variables|/Game/Inventory/Blueprints/UI2/ModulesScreen/ModulesScreen.ModulesScreen_C|GetInstalledModules _modulesscreen)
    (Utilities|Map|Add _output_get (Variables|/Game/Inventory/Blueprints/UI2/ModulesScreen/ModuleItem.ModuleItem_C|GetItem _array_element) true))
  (for _array_element_2 (Variables|/Game/Inventory/Blueprints/UI2/ModulesScreen/ModulesScreen.ModulesScreen_C|GetUninstalledModules _modulesscreen)
    (Utilities|Map|Add _output_get (Variables|/Game/Inventory/Blueprints/UI2/ModulesScreen/ModuleItemListWidget.ModuleItemListWidget_C|GetItem _array_element_2) false))
  (for _array_element_3 (Variables|/Game/Inventory/Blueprints/UI2/ConsumablesScreenContent/ConsumablesScreen.ConsumablesScreen_C|GetItemWidgets _consumablesscreen)
    (Utilities|Map|Add (Variables|/Game/Inventory/Blueprints/InventorySaver.InventorySaver_C|GetConsumables _returnvalue) (Variables|/Game/Inventory/Blueprints/UI2/ConsumablesScreenContent/ConsumablesScreenListWidget.ConsumablesScreenListWidget_C|GetItem _array_element_3) (Variables|/Game/Inventory/Blueprints/UI2/ConsumablesScreenContent/ConsumablesScreenListWidget.ConsumablesScreenListWidget_C|GetQuantity _array_element_3)))
  (bind _scrap (Default|GetScrap _consumablesscreen))
  (Variables|/Game/Inventory/Blueprints/InventorySaver.InventorySaver_C|SetScrap _returnvalue _scrap)
  (SaveGame|SaveGametoSlot _returnvalue "inventory"))