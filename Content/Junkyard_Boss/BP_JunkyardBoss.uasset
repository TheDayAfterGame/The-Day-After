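; Junkyard boss Blueprint whose Attack event plays a throw montage and signals attack end on completion or interruption.
; The montage notify spawns a volley of spike balls at the sword socket, moved by randomized forward-based vectors scaled by log distance to the player.
; Disconnected logic holds a random choice between variable-speed attack montages and a casting attack that spawns spikes around the player.
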(event EventBeginPlay
  (|CallParentFunction) ; This node is disabled and will not be called.\nDrag off pins to build functionality.
)

(event Collision|EventActorBeginOverlap
  (params (OtherActor :type Actor%20Object%20Reference)))

(event EventTick
  (params (DeltaSeconds :type Float%20%28single-precision%29))
  (|CallParentFunction DeltaSeconds) ; This node is disabled and will not be called.\nDrag off pins to build functionality.
)

(event EventAttack
  (bind _returnvalue (Game|GetPlayerCharacter 0))
  (bind _returnvalue_2 (Transformation|GetActorLocation))
  (bind _returnvalue_3 (Transformation|GetActorLocation _returnvalue))
  (bind _returnvalue_4 (Math|Vector|Distance(Vector) _returnvalue_2 _returnvalue_3))
  (bind _returnvalue_5 (Math|Float|Log _returnvalue_4 1e+01))
  (bind _returnvalue_6 (* _returnvalue_5 1e+05))
  (Animation|Montage|PlayMontage (Variables|Character|GetMesh) "/Game/Junkyard_Boss/Animations/Goalie_Throw_Montage.Goalie_Throw_Montage"
    (:OnCompleted
      (Default|CallOnAttackEnd :!label _label))
    (:OnInterrupted
      (goto _label))
    (:OnNotifyBegin
      (for _index (range 0 10)
        (bind _returnvalue_7 (Game|SpawnActorfromClass "/Game/Junkyard_Boss/AbilityAssets/BP_SpikeBall.BP_SpikeBall_C" (Math|Conversions|ToTransform(Vector) (Transformation|GetSocketLocation (Variables|Character|GetMesh) "SwordSocket")) "AlwaysSpawn" 0 0))
        (Default|Move _returnvalue_7 (* (Transformation|GetActorForwardVector) (* (Math|Random|RandomFloatinRange _returnvalue_6 (* _returnvalue_6 2.0)) (Math|Random|RandomUnitVector))))))))

(fn ConstructionScript
  (|CallParentFunction))