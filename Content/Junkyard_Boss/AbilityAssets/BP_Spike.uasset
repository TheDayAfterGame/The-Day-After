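; BP_Spike is a short-lived spike hazard actor in the Junkyard boss's ability assets.
; Its Move event snaps the cone to a lower marker, eases it up to an upper marker, holds briefly, then eases it back down and destroys the actor.
; The motion endpoints come from two destination components, animated with latent MoveComponentTo calls.
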(event Custom|Move
  (bind _cone (Variables|Default|GetCone))
  (bind _lowerdestination (Variables|Default|GetLowerDestination))
  (bind _relativelocation (Variables|/Script/Engine.SceneComponent|GetRelativeLocation _lowerdestination))
  (Transformation|SetRelativeLocation (Variables|Default|GetCone) _relativelocation false false)
  (Components|MoveComponentTo _cone (Variables|/Script/Engine.SceneComponent|GetRelativeLocation (Variables|Default|GetUpperDestination)) "0, 0, 0" true false 0.5 false)
  (Utilities|FlowControl|Delay 2.0)
  (Components|MoveComponentTo _cone _relativelocation "0, 0, 0" false true 0.5 false)
  (Actor|DestroyActor))

(fn ConstructionScript)