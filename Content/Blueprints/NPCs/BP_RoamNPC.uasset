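; Roaming NPC Blueprint that wanders around its spawn location when roaming is enabled.
; On BeginPlay it stores the spawn point, keeps max idle time at or above min, and passes the look-at-player flag to its ABP_NPCAI anim instance.
; Roam moves it to a random reachable point within a radius of that origin, then idles a random time and repeats, even after a failed move.
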(event Custom|Roam
  ;[1 1 1] Roam
  (AI|AIMoveTo self (.RandomLocation (AI|Navigation|GetRandomReachablePointinRadius (Variables|Default|GetRoam%20Vector) (Variables|RoamNPC|GetRoam%20Radius) 0 0)) 0 5.0 false
    (:OnSuccess
      _)
    (:OnFail
      _))
  (Utilities|FlowControl|Delay (Math|Random|RandomFloatinRange (Variables|RoamNPC|GetMin%20Idle%20Time) (Variables|RoamNPC|GetMax%20Idle%20Time)))
  (CallFunction|Roam))

(event EventBeginPlay
  (bind _min_idle_time (Variables|RoamNPC|GetMin%20Idle%20Time))
  (Utilities|FlowControl|Sequence
    (:then_0
      ;[1 1 1] Set Roam Vector to actor's position
      (Variables|Default|SetRoam%20Vector (Transformation|GetActorLocation)))
    (:then_1
      ;[1 1 1] Set Max Idle Time to Min Idle Time if Max Idle Time is less than Min Idle Time
      (if (< (Variables|RoamNPC|GetMax%20Idle%20Time) _min_idle_time)
        (Variables|RoamNPC|SetMax%20Idle%20Time _min_idle_time)))
    (:then_2
      ;[1 1 1] Set Looks At Player in anim class
      (bind _asabp_npcai (Utilities|Casting|CastToABP_NPCAI (Components|SkeletalMesh|GetAnimInstance (Variables|Character|GetMesh))))
      (Variables|/Game/Animations/ABP_NPCAI.ABP_NPCAI_C|SetLooks%20At%20Player _asabp_npcai (Variables|RoamNPC|GetLooks%20At%20Player)))
    (:then_3
      ;[1 1 1] Begin roaming
      (if (Variables|RoamNPC|GetIs%20Roaming)
        (CallFunction|Roam)))))

(fn ConstructionScript)