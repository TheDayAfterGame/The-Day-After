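; Quest-giver NPC that shows an interact prompt near the player, plays dialogue and advances its quest.
; Each Interact locks player movement, moves the follow camera to the NPC's view and steps through lines chosen by quest state, revealed letter by letter on Tick.
; After the last line it activates or finishes the quest and restores control.
; A colored marker shows while the quest is Completed but not yet finished.
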(event OnComponentBeginOverlap(InteractTrigger)
  (params (OverlappedComponent :type Primitive%20Component%20Object%20Reference) (OtherActor :type Actor%20Object%20Reference) (OtherComp :type Primitive%20Component%20Object%20Reference) (OtherBodyIndex :type Integer) (bFromSweep :type Boolean) (SweepResult :type Hit%20Result%20Structure%20%28by%20ref%29))
  ;[1 1 1] Create Interact Prompt when close to NPC
  (Utilities|Casting|CastToBP_ThirdPersonCharacter OtherActor)
  (CallFunction|CreatePrompt))

(event OnComponentEndOverlap(InteractTrigger)
  (params (OverlappedComponent :type Primitive%20Component%20Object%20Reference) (OtherActor :type Actor%20Object%20Reference) (OtherComp :type Primitive%20Component%20Object%20Reference) (OtherBodyIndex :type Integer))
  ;[1 1 1] Remove Interact Prompt when walking away
  (Utilities|Casting|CastToBP_ThirdPersonCharacter OtherActor)
  (CallFunction|RemovePrompt))

(event Custom|Unlock%20Movement
  ;[1 1 1] Unlock Movement
  (bind _returnvalue (Actor|GetActorOfClass "/Game/ThirdPerson/Blueprints/BP_ThirdPersonCharacter.BP_ThirdPersonCharacter_C"))
  (Pawn|Components|CharacterMovement|SetMovementMode (Variables|/Script/Engine.Character|GetCharacterMovement _returnvalue) "MOVE_Walking" 0))

(event Custom|Lock%20Movement
  ;[1 1 1] Lock Movement
  (bind _returnvalue (Actor|GetActorOfClass "/Game/ThirdPerson/Blueprints/BP_ThirdPersonCharacter.BP_ThirdPersonCharacter_C"))
  (Pawn|Components|CharacterMovement|SetMovementMode (Variables|/Script/Engine.Character|GetCharacterMovement _returnvalue) "MOVE_None" 0))

(event Custom|Lock%20Camera
  ;[1 1 1] Lock Camera
  (bind _returnvalue (Actor|GetActorOfClass "/Game/ThirdPerson/Blueprints/BP_ThirdPersonCharacter.BP_ThirdPersonCharacter_C"))
  (Transformation|AttachComponentToComponent (Variables|/Game/ThirdPerson/Blueprints/BP_ThirdPersonCharacter.BP_ThirdPersonCharacter_C|GetFollowCamera _returnvalue) (Variables|Default|GetCamera%20Location) "None" "KeepRelative" "KeepRelative" "KeepRelative" true))

(event Custom|Create%20Text%20Box
  ;[1 1 1] Create Text Box
  (bind _returnvalue (UserInterface|CreateWidget "/Game/Blueprints/NPCs/WB_Dialogue.WB_Dialogue_C" (Game|GetPlayerController 0)))
  (bind _output_get (Variables|Default|SetUI _returnvalue))
  (UserInterface|Viewport|AddtoViewport _output_get 0)
  (Rendering|Components|TextRender|SetText (Variables|/Game/Blueprints/NPCs/WB_Dialogue.WB_Dialogue_C|GetName (Variables|Default|GetUI)) (Utilities|Text|ToText(String) (Variables|QuestNPC|GetName))))

(event Custom|Display%20text
  (params (Prompt :type Array%20of%20Strings) (Prompt%20Index :type Integer) (Text%20Index :type Integer))
  ;[1 1 1] Display Text
  (Rendering|Components|TextRender|SetText (Variables|/Game/Blueprints/NPCs/WB_Dialogue.WB_Dialogue_C|GetDialogue (Variables|Default|GetUI)) (Utilities|Text|ToText(String) (Utilities|String|GetSubstring (Utilities|Array|Get(acopy) Prompt Prompt%20Index) 0 Text%20Index))))

(event Custom|Unlock%20Camera
  ;[1 1 1] Lock Camera
  (bind _returnvalue (Actor|GetActorOfClass "/Game/ThirdPerson/Blueprints/BP_ThirdPersonCharacter.BP_ThirdPersonCharacter_C"))
  (Transformation|AttachComponentToComponent (Variables|/Game/ThirdPerson/Blueprints/BP_ThirdPersonCharacter.BP_ThirdPersonCharacter_C|GetFollowCamera _returnvalue) (Variables|/Game/ThirdPerson/Blueprints/BP_ThirdPersonCharacter.BP_ThirdPersonCharacter_C|GetCameraBoom _returnvalue) "None" "KeepRelative" "KeepRelative" "KeepRelative" true))

(event Custom|Update%20Quest%20State
  (bind _quest_id (Variables|QuestNPC|GetQuest%20ID))
  ;[1 1 1] Update Quest State
  (switch Utilities|FlowControl|Switch|SwitchonE_QuestState (.State (Utilities|Struct|BreakS_Quest (CallFunction|GetQuest (Variables|QuestNPC|GetQuest%20ID))))
    (:NewEnumerator0
      (CallFunction|ActivateQuest _quest_id))
    (:NewEnumerator2
      (CallFunction|FinishQuest _quest_id))))

(event Custom|Create%20Prompt
  ;[1 1 1] Create Interact Prompt
  (if (and (Utilities|Enum|NotEqual(Enum) (.State (Utilities|Struct|BreakS_Quest (CallFunction|GetQuest (Variables|QuestNPC|GetQuest%20ID)))) "NewEnumerator5") (not (Variables|Default|GetInteract%20Prompt%20Is%20Shown?)))
    (bind _returnvalue (UserInterface|CreateWidget "/Game/Blueprints/NPCs/WB_InteractPrompt.WB_InteractPrompt_C" (Game|GetPlayerController 0)))
    (bind _output_get (Variables|Default|SetPrompt _returnvalue))
    (UserInterface|Viewport|AddtoViewport _output_get 0)
    (Variables|Default|SetInteract%20Prompt%20Is%20Shown? true)))

(event Custom|Remove%20Prompt
  ;[1 1 1] Remove Interact Prompt
  (if (Variables|Default|GetInteract%20Prompt%20Is%20Shown?)
    (Widget|RemovefromParent (Variables|Default|GetPrompt))
    (Variables|Default|SetInteract%20Prompt%20Is%20Shown? false)))

(event Custom|Animation%20Tick
  (params (Delta%20Seconds :type Float%20%28double-precision%29))
  ;[1 1 1] Animation for dialogue prompts
  (if (Variables|Default|GetIs%20Iterating)
    (bind _output_get (Variables|Default|SetIterate%20Timer (- (Variables|Default|GetIterate%20Timer) Delta%20Seconds)))
    (if (<= _output_get 0.0)
      (Variables|Default|SetIterate%20Timer (/ (Variables|QuestNPC|GetText%20Animation%20Speed) 1e+02))
      (bind _result (Math|Integer|IncrementInt (Variables|Default|GetText%20Index))
        (:%20%20
          (bind _prompt (CallFunction|GetCurrentPrompt))
          (CallFunction|DisplayText _prompt (Variables|Default|GetDialogue%20Index) _result))))
    (else
      (Variables|Default|SetIterate%20Timer 0.0))))

(event EventBeginPlay
  ;[1 1 1] Set Looks At Player in anim class
  (bind _asabp_npcai (Utilities|Casting|CastToABP_NPCAI (Components|SkeletalMesh|GetAnimInstance (Variables|Character|GetMesh))))
  (Variables|/Game/Animations/ABP_NPCAI.ABP_NPCAI_C|SetLooks%20At%20Player _asabp_npcai (Variables|QuestNPC|GetLooks%20At%20Player))
  ;[1 1 1] Set marker color
  (Appearance|SetColorandOpacity (UserInterface|GetWidget (Variables|Default|GetMarker)) (Math|Conversions|ToLinearColor(Color) (Variables|QuestNPC|GetMarker%20Color)) :!class /Script/UMG.UserWidget))

(event EventInteract
  ;[1 1 1] Check if quest is not finished
  (if (Utilities|Enum|NotEqual(Enum) (.State (Utilities|Struct|BreakS_Quest (CallFunction|GetQuest (Variables|QuestNPC|GetQuest%20ID)))) "NewEnumerator5")
    ;[1 1 1] Setup for iteration
    (Utilities|FlowControl|Sequence
      (:then_0
        (CallFunction|LockMovement))
      (:then_1
        (CallFunction|LockCamera))
      (:then_2
        (Math|Integer|IncrementInt (Variables|Default|GetDialogue%20Index)))
      (:then_3
        (Variables|Default|SetText%20Index 0))
      (:then_4
        (Variables|Default|SetIterate%20Timer 0.0))
      (:then_5
        (CallFunction|RemovePrompt))
      (:then_6
        (Variables|Default|SetIs%20Iterating true)
        ;[1 1 1] Iterate through dialogue prompt
        (bind _prompt (CallFunction|GetCurrentPrompt))
        (if (< (Variables|Default|GetDialogue%20Index) (Utilities|Array|Length _prompt))
          (if (not (> (Variables|Default|GetDialogue%20Index) 0))
            (CallFunction|CreateTextBox))
          (else
            (Widget|RemovefromParent (Variables|Default|GetUI))
            (Variables|Default|SetDialogue%20Index -1)
            (CallFunction|UpdateQuestState)
            (CallFunction|UnlockMovement)
            (CallFunction|UnlockCamera)
            (CallFunction|CreatePrompt)
            (Variables|Default|SetIs%20Iterating false)))))))

(event EventTick
  (params (DeltaSeconds :type Float%20%28single-precision%29))
  (CallFunction|AnimationTick DeltaSeconds)
  ;[1 1 1] Update marker visibility
  (Rendering|SetVisibility (Variables|Default|GetMarker) (Utilities|Enum|Equal(Enum) (.State (Utilities|Struct|BreakS_Quest (CallFunction|GetQuest (Variables|QuestNPC|GetQuest%20ID)))) "NewEnumerator2") false))

(fn ConstructionScript)

(fn GetCurrentPrompt
  (switch Utilities|FlowControl|Switch|SwitchonE_QuestState (.State (Utilities|Struct|BreakS_Quest (CallFunction|GetQuest (Variables|QuestNPC|GetQuest%20ID))))
    (:NewEnumerator0
      (return (Variables|QuestNPC|GetQuest%20Prompt)))
    (:NewEnumerator1
      (return (Variables|QuestNPC|GetQuest%20Doing%20Prompt)))
    (:NewEnumerator2
      (return (Variables|QuestNPC|GetQuest%20Complete%20Prompt)))))