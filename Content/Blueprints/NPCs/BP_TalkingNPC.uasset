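; Talking NPC that shows an interact prompt when the player enters its trigger and runs a multi-line dialogue on Interact.
; Each interaction locks the player's movement, attaches their camera to the NPC's camera point and advances the line, restoring both after the last one.
; Tick types each line out character by character into a dialogue widget.
; BeginPlay passes the look-at-player setting to the NPC anim Blueprint.
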(event OnComponentBeginOverlap(InteractTrigger)
  (params (OverlappedComponent :type Primitive%20Component%20Object%20Reference) (OtherActor :type Actor%20Object%20Reference) (OtherComp :type Primitive%20Component%20Object%20Reference) (OtherBodyIndex :type Integer) (bFromSweep :type Boolean) (SweepResult :type Hit%20Result%20Structure%20%28by%20ref%29))
  ;[1 1 1] Create Interact Prompt when close to NPC
  (Utilities|Casting|CastToBP_ThirdPersonCharacter OtherActor)
  (CallFunction|CreatePrompt))

(event OnComponentEndOverlap(InteractTrigger)
  (params (OverlappedComponent :type Primitive%20Component%20Object%20Reference) (OtherActor :type Actor%20Object%20Reference) (OtherComp :type Primitive%20Component%20Object%20Reference) (OtherBodyIndex :type Integer))
  ;[1 1 1] Remove Interact Prompt when walking away
  (Utilities|Casting|CastToBP_ThirdPersonCharacter OtherActor)
  (CallFunction|RemovePrompt))

(event Custom|Unlock%20Movement
  ;[1 1 1] Unlock Movement
  (bind _returnvalue (Actor|GetActorOfClass "/Game/ThirdPerson/Blueprints/BP_ThirdPersonCharacter.BP_ThirdPersonCharacter_C"))
  (Pawn|Components|CharacterMovement|SetMovementMode (Variables|/Script/Engine.Character|GetCharacterMovement _returnvalue) "MOVE_Walking" 0))

(event Custom|Lock%20Movement
  ;[1 1 1] Lock Movement
  (bind _returnvalue (Actor|GetActorOfClass "/Game/ThirdPerson/Blueprints/BP_ThirdPersonCharacter.BP_ThirdPersonCharacter_C"))
  (Pawn|Components|CharacterMovement|SetMovementMode (Variables|/Script/Engine.Character|GetCharacterMovement _returnvalue) "MOVE_None" 0))

(event Custom|Lock%20Camera
  ;[1 1 1] Lock Camera
  (bind _returnvalue (Actor|GetActorOfClass "/Game/ThirdPerson/Blueprints/BP_ThirdPersonCharacter.BP_ThirdPersonCharacter_C"))
  (Transformation|AttachComponentToComponent (Variables|/Game/ThirdPerson/Blueprints/BP_ThirdPersonCharacter.BP_ThirdPersonCharacter_C|GetFollowCamera _returnvalue) (Variables|Default|GetCamera%20Location) "None" "KeepRelative" "KeepRelative" "KeepRelative" true))

(event Custom|Create%20Text%20Box
  ;[1 1 1] Create Text Box
  (bind _returnvalue (UserInterface|CreateWidget "/Game/Blueprints/NPCs/WB_Dialogue.WB_Dialogue_C" (Game|GetPlayerController 0)))
  (bind _output_get (Variables|Default|SetUI _returnvalue))
  (UserInterface|Viewport|AddtoViewport _output_get 0)
  (Rendering|Components|TextRender|SetText (Variables|/Game/Blueprints/NPCs/WB_Dialogue.WB_Dialogue_C|GetName (Variables|Default|GetUI)) (Utilities|Text|ToText(String) (Variables|TalkingNPC|GetName))))

(event Custom|Display%20text
  (params (Prompt%20Index :type Integer) (Text%20Index :type Integer))
  ;[1 1 1] Display Text
  (Rendering|Components|TextRender|SetText (Variables|/Game/Blueprints/NPCs/WB_Dialogue.WB_Dialogue_C|GetDialogue (Variables|Default|GetUI)) (Utilities|Text|ToText(String) (Utilities|String|GetSubstring (Utilities|Array|Get(acopy) (Variables|TalkingNPC|GetDialogue%20Prompt) Prompt%20Index) 0 Text%20Index))))

(event Custom|Unlock%20Camera
  ;[1 1 1] Lock Camera
  (bind _returnvalue (Actor|GetActorOfClass "/Game/ThirdPerson/Blueprints/BP_ThirdPersonCharacter.BP_ThirdPersonCharacter_C"))
  (Transformation|AttachComponentToComponent (Variables|/Game/ThirdPerson/Blueprints/BP_ThirdPersonCharacter.BP_ThirdPersonCharacter_C|GetFollowCamera _returnvalue) (Variables|/Game/ThirdPerson/Blueprints/BP_ThirdPersonCharacter.BP_ThirdPersonCharacter_C|GetCameraBoom _returnvalue) "None" "KeepRelative" "KeepRelative" "KeepRelative" true))

(event Custom|Create%20Prompt
  ;[1 1 1] Create Interact Prompt
  (if (not (Variables|Default|GetInteract%20Prompt%20Is%20Shown?))
    (bind _returnvalue (UserInterface|CreateWidget "/Game/Blueprints/NPCs/WB_InteractPrompt.WB_InteractPrompt_C" (Game|GetPlayerController 0)))
    (bind _output_get (Variables|Default|SetPrompt _returnvalue))
    (UserInterface|Viewport|AddtoViewport _output_get 0)
    (Variables|Default|SetInteract%20Prompt%20Is%20Shown? true)))

(event Custom|Remove%20Prompt
  ;[1 1 1] Remove Interact Prompt
  (if (Variables|Default|GetInteract%20Prompt%20Is%20Shown?)
    (Widget|RemovefromParent (Variables|Default|GetPrompt))
    (Variables|Default|SetInteract%20Prompt%20Is%20Shown? false)))

(event EventBeginPlay
  ;[1 1 1] Set Looks At Player in anim class
  (bind _asabp_npcai (Utilities|Casting|CastToABP_NPCAI (Components|SkeletalMesh|GetAnimInstance (Variables|Character|GetMesh))))
  (Variables|/Game/Animations/ABP_NPCAI.ABP_NPCAI_C|SetLooks%20At%20Player _asabp_npcai (Variables|TalkingNPC|GetLooks%20At%20Player)))

(event EventInteract
  ;[1 1 1] Setup for iteration
  (Utilities|FlowControl|Sequence
    (:then_0
      (CallFunction|LockMovement))
    (:then_1
      (CallFunction|LockCamera))
    (:then_2
      (Math|Integer|IncrementInt (Variables|Default|GetDialogue%20Index)))
    (:then_3
      (Variables|Default|SetText%20Index 0))
    (:then_4
      (Variables|Default|SetIterate%20Timer 0.0))
    (:then_5
      (CallFunction|RemovePrompt))
    (:then_6
      (Variables|Default|SetIs%20Iterating true)
      ;[1 1 1] Iterate through dialogue prompt
      (if (< (Variables|Default|GetDialogue%20Index) (Utilities|Array|Length (Variables|TalkingNPC|GetDialogue%20Prompt)))
        (if (not (> (Variables|Default|GetDialogue%20Index) 0))
          (CallFunction|CreateTextBox))
        (else
          (Widget|RemovefromParent (Variables|Default|GetUI))
          (Variables|Default|SetDialogue%20Index -1)
          (CallFunction|UnlockMovement)
          (CallFunction|UnlockCamera)
          (CallFunction|CreatePrompt)
          (Variables|Default|SetIs%20Iterating false))))))

(event EventTick
  (params (DeltaSeconds :type Float%20%28single-precision%29))
  ;[1 1 1] Animation for dialogue prompts
  (if (Variables|Default|GetIs%20Iterating)
    (bind _output_get (Variables|Default|SetIterate%20Timer (- (Variables|Default|GetIterate%20Timer) DeltaSeconds)))
    (if (<= _output_get 0.0)
      (Variables|Default|SetIterate%20Timer (/ (Variables|TalkingNPC|GetText%20Animation%20Speed) 1e+02))
      (bind _result (Math|Integer|IncrementInt (Variables|Default|GetText%20Index))
        (:%20%20
          (CallFunction|DisplayText (Variables|Default|GetDialogue%20Index) _result))))
    (else
      (Variables|Default|SetIterate%20Timer 0.0))))

(fn ConstructionScript)