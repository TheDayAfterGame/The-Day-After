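; Blueprint function library for the quest system, giving global access to look up, change and describe quests by ID.
; It finds BP_QuestManager with GetActorOfClass, edits the matching struct in its Quests array and saves after each state change.
; Finishing a quest also grants scrap and item rewards to the third-person character's inventory and removes any required items.
; A formatter builds display text from name, description, rewards and status.
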(fn GetQuest
  (params (Quest%20ID :type Integer))
  (for _array_element (Variables|/Game/Blueprints/QuestSystem/BP_QuestManager.BP_QuestManager_C|GetQuests (CallFunction|GetQuestManager))
    (if (== (.QuestID (Utilities|Struct|BreakS_Quest _array_element)) Quest%20ID)
      (return _array_element))))

(fn GetAllQuests
  (return (Variables|/Game/Blueprints/QuestSystem/BP_QuestManager.BP_QuestManager_C|GetQuests (CallFunction|GetQuestManager))))

(fn SetQuestState
  (params (Quest%20ID :type Integer) (State :type E_QuestState%20Enum :default "NewEnumerator0"))
  (bind _quest_manager (CallFunction|GetQuestManager))
  (bind _quests (Variables|/Game/Blueprints/QuestSystem/BP_QuestManager.BP_QuestManager_C|GetQuests _quest_manager))
  (for (_array_element _array_index) _quests
    (if (== (.QuestID (Utilities|Struct|BreakS_Quest _array_element)) Quest%20ID)
      (Utilities|Struct|SetmembersinS_Quest (Utilities|Array|Get(acopy) _quests _array_index) State)
      (CallFunction|SaveQuests)
      (return))))

(fn ActivateQuest
  (params (Quest%20ID :type Integer))
  (CallFunction|SetQuestState Quest%20ID "NewEnumerator1"))

(fn CompleteQuest
  (params (Quest%20ID :type Integer))
  (CallFunction|SetQuestState Quest%20ID "NewEnumerator2"))

(fn FinishQuest
  (params (Quest%20ID :type Integer))
  (bind _quest (CallFunction|GetQuest Quest%20ID))
  (bind _quest_2 (CallFunction|GetQuest Quest%20ID))
  (bind _itemreward (Utilities|Struct|BreakS_Quest _quest))
  (bind (_itemtoget _amount) (Utilities|Struct|BreakS_Quest _quest_2))
  (Utilities|FlowControl|Sequence
    (:then_0
      (CallFunction|SetQuestState Quest%20ID "NewEnumerator5"))
    (:then_1
      ;[1 1 1] Give Scrap Reward
      (bind _returnvalue (Actor|GetActorOfClass 0 "/Game/ThirdPerson/Blueprints/BP_ThirdPersonCharacter.BP_ThirdPersonCharacter_C"))
      (Default|AddScrap (Variables|/Game/ThirdPerson/Blueprints/BP_ThirdPersonCharacter.BP_ThirdPersonCharacter_C|GetInventory _returnvalue) (.ScrapReward (Utilities|Struct|BreakS_Quest (CallFunction|GetQuest Quest%20ID)))))
    (:then_2
      ;[1 1 1] Give Item Rewrad
      (if (not (Utilities|Enum|Equal(Enum) _itemreward "NewEnumerator7"))
        (bind _returnvalue_2 (Actor|GetActorOfClass 0 "/Game/ThirdPerson/Blueprints/BP_ThirdPersonCharacter.BP_ThirdPersonCharacter_C"))
        (Default|Add (Variables|/Game/ThirdPerson/Blueprints/BP_ThirdPersonCharacter.BP_ThirdPersonCharacter_C|GetInventory _returnvalue_2) _itemreward)))
    (:then_3
      ;[1 1 1] Try to remove Item To Get
      (if (not (Utilities|Enum|Equal(Enum) _itemtoget "NewEnumerator7"))
        (bind _returnvalue_3 (Actor|GetActorOfClass 0 "/Game/ThirdPerson/Blueprints/BP_ThirdPersonCharacter.BP_ThirdPersonCharacter_C"))
        (Default|Remove (Variables|/Game/ThirdPerson/Blueprints/BP_ThirdPersonCharacter.BP_ThirdPersonCharacter_C|GetInventory _returnvalue_3) _itemtoget _amount)))))

(fn QuesttoString
  (params (Quest%20ID :type Integer))
  (bind _quest (CallFunction|GetQuest Quest%20ID))
  (bind (_name _description _itemtoget _scrapreward _itemreward _state) (Utilities|Struct|BreakS_Quest _quest))
  (Utilities|FlowControl|Sequence
    (:then_0
      ;[1 1 1] Add name and description
      (LocalVariables|SetOutput (Utilities|String|Append _name " 
" _description)))
    (:then_1
      ;[1 1 1] Add scrap reward if one
      (if (>= _scrapreward 0)
        (LocalVariables|SetOutput (Utilities|String|Append (LocalVariables|GetOutput) " 
Scrap reward: " (Utilities|String|ToString(Integer) _scrapreward)))))
    (:then_2
      ;[1 1 1] Add item reward if one
      (if (not (Utilities|Enum|Equal(Enum) _itemreward "NewEnumerator7"))
        (LocalVariables|SetOutput (Utilities|String|Append (LocalVariables|GetOutput) " 
Item reward: " (Utilities|String|EnumtoString _itemreward)))))
    (:then_3
      ;[1 1 1] Add status
      (LocalVariables|SetOutput (Utilities|String|Append (LocalVariables|GetOutput) " 
Status: " (Utilities|String|EnumtoString _state) " 
 
")))
    (:then_4
      ;[1 1 1] Return
      (return (LocalVariables|GetOutput)))))

(fn GetQuestManager
  (bind _returnvalue (Actor|GetActorOfClass 0 "/Game/Blueprints/QuestSystem/BP_QuestManager.BP_QuestManager_C"))
  (return _returnvalue))

(fn SaveQuests
  (Default|SaveQuests (CallFunction|GetQuestManager)))