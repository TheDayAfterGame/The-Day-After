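; Quest marker actor that displays a colored widget in the world while its linked quest is active.
; BeginPlay tints the Marker widget with the Color variable.
; Each tick rotates the root to face the BP_ThirdPersonCharacter's follow camera, billboard style.
; Tick also polls the state of the quest matching QuestID and hides the marker unless that quest is active.
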(event EventBeginPlay
  ;[1 1 1] Set sprite color
  (Appearance|SetColorandOpacity (UserInterface|GetWidget (Variables|Default|GetMarker)) (Math|Conversions|ToLinearColor(Color) (Variables|QuestMarker|GetColor)) :!class /Script/UMG.UserWidget))

(event EventTick
  (params (DeltaSeconds :type Float%20%28single-precision%29))
  (bind _defaultsceneroot (Variables|Default|GetDefaultSceneRoot))
  (Utilities|FlowControl|Sequence
    (:then_0
      ;[1 1 1] Look at camera
      (bind _asbp_third_person_character (Utilities|Casting|CastToBP_ThirdPersonCharacter (Game|Player|GetPlayerPawn 0)))
      (Transformation|SetWorldRotation _defaultsceneroot (Math|Rotator|FindLookatRotation (Transformation|GetWorldLocation _defaultsceneroot) (Transformation|GetWorldLocation (Variables|/Game/ThirdPerson/Blueprints/BP_ThirdPersonCharacter.BP_ThirdPersonCharacter_C|GetFollowCamera _asbp_third_person_character))) false false))
    (:then_1
      ;[1 1 1] Show when quest is active
      (Development|SetHiddeninGame (Variables|Default|GetMarker) (not (Utilities|Enum|Equal(Enum) (.State (Utilities|Struct|BreakS_Quest (CallFunction|GetQuest (Variables|QuestMarker|GetQuest%20ID)))) "NewEnumerator1")) false))))

(fn ConstructionScript)