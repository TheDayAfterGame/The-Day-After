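; Quest manager that holds the game's quest list, persists it to a save slot and tracks item quests.
; On BeginPlay it loads saved quests, falling back to DT_Quests when a reset flag is set or no saved quests exist, then saves.
; Every Tick it checks the player's inventory for item quests in eligible states, calling CompleteQuest when the required amount is held, otherwise ActivateQuest.
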(event Custom|Save%20Quests
  ;[1 1 1] Save Game
  (bind _returnvalue (SaveGame|CreateSaveGameObject "/Game/Blueprints/QuestSystem/SG_QuestSaveSystem.SG_QuestSaveSystem_C"))
  (bind _output_get (Variables|Default|SetSave%20Game%20Instance _returnvalue))
  (Variables|/Game/Blueprints/QuestSystem/SG_QuestSaveSystem.SG_QuestSaveSystem_C|SetQuests _output_get (Variables|Default|GetQuests))
  (|AsyncSaveGametoSlot _output_get "quests"))

(event Custom|Load%20Game
  ;[1 1 1] Load Game
  (if (Variables|QuestManager|GetReset%20Quest%20States%20On%20Play)
    (CallFunction|ReadfromDataTable :!label _label)
    (else
      (bind _returnvalue (SaveGame|LoadGamefromSlot "quests"))
      (bind _assg_quest_save_system (Utilities|Casting|CastToSG_QuestSaveSystem _returnvalue)
        (:then
          (if (Utilities|Array|IsEmpty (Variables|/Game/Blueprints/QuestSystem/SG_QuestSaveSystem.SG_QuestSaveSystem_C|GetQuests _assg_quest_save_system))
            (goto _label)
            (else
              (Variables|Default|SetQuests (Variables|/Game/Blueprints/QuestSystem/SG_QuestSaveSystem.SG_QuestSaveSystem_C|GetQuests _assg_quest_save_system)))))
        (:CastFailed
          (goto _label))))))

(event Custom|Read%20From%20Data%20Table
  ;[1 1 1] Read Quests From Data Table
  (bind _outrownames (DataTable|GetDataTableRowNames "/Game/Blueprints/QuestSystem/DT_Quests.DT_Quests"))
  (for _array_element _outrownames
    (bind _returnvalue (Utilities|GetDataTableRow "/Game/Blueprints/QuestSystem/DT_Quests.DT_Quests" _array_element)
      (:then
        (Utilities|Array|Add (Variables|Default|GetQuests) _returnvalue))))
  (CallFunction|SaveQuests))

(event EventBeginPlay
  (CallFunction|LoadGame))

(event EventTick
  (params (DeltaSeconds :type Float%20%28single-precision%29))
  ;[1 1 1] Update Item Quests
  (for _array_element (Variables|Default|GetQuests)
    (if (Math|Boolean|ANDBoolean (Utilities|Enum|Equal(Enum) (.Type (Utilities|Struct|BreakS_Quest _array_element)) "NewEnumerator1") (Utilities|Enum|NotEqual(Enum) (.State (Utilities|Struct|BreakS_Quest _array_element)) "NewEnumerator0") (Utilities|Enum|NotEqual(Enum) (.State (Utilities|Struct|BreakS_Quest _array_element)) "NewEnumerator5"))
      (bind _returnvalue (Actor|GetActorOfClass "/Game/ThirdPerson/Blueprints/BP_ThirdPersonCharacter.BP_ThirdPersonCharacter_C"))
      (bind _numitems (Default|HasItem (Variables|/Game/ThirdPerson/Blueprints/BP_ThirdPersonCharacter.BP_ThirdPersonCharacter_C|GetInventory _returnvalue) (.ItemToGet (Utilities|Struct|BreakS_Quest _array_element))))
      (if (>= _numitems (.Amount (Utilities|Struct|BreakS_Quest _array_element)))
        (CallFunction|CompleteQuest (.QuestID (Utilities|Struct|BreakS_Quest _array_element)))
        (else
          (CallFunction|ActivateQuest (.QuestID (Utilities|Struct|BreakS_Quest _array_element))))))))

(fn ConstructionScript)