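; Health component that tracks its owner's health and shows it on a world-space WB_HealthBar widget created at BeginPlay.
; TakeDamage drops the main bar instantly, while a trailing recent-damage bar eases down after a delay.
; Tick drives that easing, fades the bar out after a hit-free delay, and turns the widget toward the camera.
; Distance culling and the zero-health OnDestroy call, meant to destroy the owner, are not wired up.
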(event Custom|HandleOnDestroy
  (Actor|DestroyActor (Components|GetOwner)))

(event EventBeginPlay
  (bind _output_get (Variables|HealthBar|SetHealth (Variables|HealthBar|GetMaxHealth)))
  (bind _output_get_2 (Variables|HealthBar|SetPreviousHealth _output_get))
  (Variables|HealthBar|SetPreviousHealthStart _output_get_2)
  (bind _returnvalue (Game|AddComponentbyClass (Components|GetOwner) "/Script/UMG.WidgetComponent" false (|EmptyTransform)))
  (bind _returnvalue_2 (UserInterface|CreateWidget "/Game/Widgets/WB_HealthBar.WB_HealthBar_C"))
  (UserInterface|SetWidget _returnvalue _returnvalue_2)
  (Collision|SetCollisionEnabled _returnvalue "NoCollision")
  (Variables|Default|SetWidget _returnvalue)
  (EventDispatchers|BindEventtoOnDestroy (delegate Custom|HandleOnDestroy))
  (CallFunction|UpdateHealthBarOpacity)
  (CallFunction|UpdateRecentDamageBar))

(event EventTick
  (params (DeltaSeconds :type Float%20%28single-precision%29))
  (|InterpolateHealthBar DeltaSeconds
    (:OutputPin
      (Transformation|SetWorldLocationAndRotation (Variables|Default|GetWidget) (.ReturnValue (|GetWidgetNewLocation)) (|GetWidgetNewRotation (Game|GetPlayerCameraManager 0)) false true))))

(fn UpdateHealthBar
  (bind _health (Variables|HealthBar|GetHealth))
  (bind _maxhealth (Variables|HealthBar|GetMaxHealth))
  (bind _returnvalue (/ _health _maxhealth))
  (bind _aswb_health_bar (Utilities|Casting|CastToWB_HealthBar (UserInterface|GetWidget (Variables|Default|GetWidget))))
  (Progress|SetPercent (Variables|/Game/Widgets/WB_HealthBar.WB_HealthBar_C|GetProgressBar _aswb_health_bar) _returnvalue)
  (if (<= _returnvalue 0.0)
    _))

(fn TakeDamage
  (params (Damage :type Float%20%28double-precision%29))
  (Variables|HealthBar|SetHealth (- (Variables|HealthBar|GetHealth) Damage))
  (Variables|HealthBar|SetTimeSinceLastHit 0.0)
  (Variables|HealthBar|SetPreviousHealthStart (Variables|HealthBar|GetPreviousHealth))
  (CallFunction|UpdateHealthBarOpacity)
  (CallFunction|UpdateHealthBar))

(fn UpdateRecentDamageBar
  (bind _aswb_health_bar (Utilities|Casting|CastToWB_HealthBar (UserInterface|GetWidget (Variables|Default|GetWidget))))
  (Progress|SetPercent (Variables|/Game/Widgets/WB_HealthBar.WB_HealthBar_C|GetProgressBarBackground _aswb_health_bar) (/ (Variables|HealthBar|GetPreviousHealth) (Variables|HealthBar|GetMaxHealth))))

(fn UpdateHealthBarOpacity
  (bind _timesincelasthit (Variables|HealthBar|GetTimeSinceLastHit))
  (bind _fadeoutdelay (Variables|HealthBar|GetFadeOutDelay))
  (bind _returnvalue (- _timesincelasthit _fadeoutdelay))
  (Widget|SetRenderOpacity (UserInterface|GetWidget (Variables|Default|GetWidget)) (Math|Float|SelectFloat (Class|KismetMathLibrary|FInterpEaseinOut 1.0 0.0 (Math|Float|Min(Float) (/ _returnvalue (Variables|HealthBar|GetFadeOutDuration)) 1.0) 1.0) 1.0 (>= _returnvalue 0.0))))

(fn DisableHealthBar
  (Widget|SetRenderOpacity (UserInterface|GetWidget (Variables|Default|GetWidget)) 0.0))