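; Attack component for the enemy mage that fires a dark energy projectile and damages the player on impact.
; MagicSpell spawns the projectile at a given transform, binds its impact event and sets it to ignore the owner.
; A hit on the third-person character applies damage, reports it to AI perception and plays a camera shake.
; OnAttackEnded fires only after such a hit, not on other impacts.
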(event Custom|MagicSpell
  (params (SpawnTransform :type Transform) (BaseDamage :type Float%20%28single-precision%29))
  (bind _returnvalue (Game|SpawnActorfromClass "/Game/Characters/Projectiles/BP_Projectile_DarkEnergy.BP_Projectile_DarkEnergy_C" SpawnTransform "Undefined" (Components|GetOwner) 1e+03 0.0 0 false 0))
  (EventDispatchers|AssignOnProjectileImpact _returnvalue (delegate Custom|OnProjectileHit))
  (Collision|IgnoreActorwhenMoving (Variables|/Game/Characters/Projectiles/BP_Projectile_Base.BP_Projectile_Base_C|GetBoxCollision _returnvalue) (Components|GetOwner) true))

(event Custom|OnProjectileHit
  (params (OtherActor :type Actor%20Object%20Reference) (Hit :type Hit%20Result%20Structure))
  (bind _returnvalue (Components|GetOwner))
  (Utilities|Casting|CastToBP_ThirdPersonCharacter OtherActor)
  (Game|Damage|ApplyDamage OtherActor (stale Custom|MagicSpell BaseDamage) (AI|GetAIController _returnvalue) (stale Custom|MagicSpell _returnvalue))
  (Class|AISenseDamage|ReportDamageEvent OtherActor _returnvalue (stale Custom|MagicSpell BaseDamage) (Transformation|GetActorLocation _returnvalue) "0, 0, 0" "None")
  (Camera|PlayWorldCameraShake "/Game/Enemies/AI/BP_HitShake.BP_HitShake_C" (.Location (Collision|BreakHitResult Hit)) 0.0 2e+03)
  (Default|CallOnAttackEnded))

(event EventBeginPlay)

(event EventTick
  (params (DeltaSeconds :type Float%20%28single-precision%29)))