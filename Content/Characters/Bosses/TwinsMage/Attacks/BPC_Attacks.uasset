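; Attack component for the TwinsMage boss, providing three projectile spells and a summon.
; Dark Energy, Thunder Ball and player-homing Frenzied Fire projectiles ignore their owner and bind impact callbacks.
; Player hits apply damage, report it to AI perception, shake the camera and fire OnAttackEnded; other impacts do not end the attack.
; Summon spawns a BP_Mage with its behavior tree, then fires OnAttackEnded next tick.
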(event Custom|Summon
  (params (SpawnTransform :type Transform))
  (AI|SpawnAIFromClass "/Game/Enemies/BP_Mage.BP_Mage_C" "/Game/Enemies/AI/BehaviorTrees/BT_Enemy_Mage.BT_Enemy_Mage" (.location SpawnTransform) (.rotation SpawnTransform) false 0)
  (Utilities|FlowControl|DelayUntilNextTick)
  (Default|CallOnAttackEnded))

(event Custom|CustomEvent_2
  (params (OtherActor :type Actor%20Object%20Reference) (Hit :type Hit%20Result%20Structure))
  (bind _returnvalue (Components|GetOwner))
  (Utilities|Casting|CastToBP_ThirdPersonCharacter OtherActor)
  (Game|Damage|ApplyDamage OtherActor (stale Custom|FrenziedFire BaseDamage) (AI|GetAIController _returnvalue) (stale Custom|FrenziedFire _returnvalue))
  (Class|AISenseDamage|ReportDamageEvent OtherActor _returnvalue (stale Custom|FrenziedFire BaseDamage) (Transformation|GetActorLocation _returnvalue) "0, 0, 0" "None")
  (Camera|PlayWorldCameraShake "/Game/Enemies/AI/BP_HitShake.BP_HitShake_C" (.Location (Collision|BreakHitResult Hit)) 0.0 2e+03)
  (Default|CallOnAttackEnded))

(event Custom|MagicSpell
  (params (SpawnTransform :type Transform) (BaseDamage :type Float%20%28single-precision%29))
  (bind _returnvalue (Game|SpawnActorfromClass "/Game/Characters/Projectiles/BP_Projectile_DarkEnergy.BP_Projectile_DarkEnergy_C" SpawnTransform "Undefined" (Components|GetOwner) 2.5e+03 0.0 0 false 0))
  (EventDispatchers|AssignOnProjectileImpact _returnvalue (delegate Custom|OnProjectileHit))
  (Collision|IgnoreActorwhenMoving (Variables|/Game/Characters/Projectiles/BP_Projectile_Base.BP_Projectile_Base_C|GetBoxCollision _returnvalue) (Components|GetOwner) true))

(event Custom|OnProjectileHit
  (params (OtherActor :type Actor%20Object%20Reference) (Hit :type Hit%20Result%20Structure))
  (bind _returnvalue (Components|GetOwner))
  (Utilities|Casting|CastToBP_ThirdPersonCharacter OtherActor)
  (Game|Damage|ApplyDamage OtherActor (stale Custom|MagicSpell BaseDamage) (AI|GetAIController _returnvalue) (stale Custom|MagicSpell _returnvalue))
  (Class|AISenseDamage|ReportDamageEvent OtherActor _returnvalue (stale Custom|MagicSpell BaseDamage) (Transformation|GetActorLocation _returnvalue) "0, 0, 0" "None")
  (Camera|PlayWorldCameraShake "/Game/Enemies/AI/BP_HitShake.BP_HitShake_C" (.Location (Collision|BreakHitResult Hit)) 0.0 2e+03)
  (Default|CallOnAttackEnded))

(event Custom|ThunderSpell
  (params (SpawnTransform :type Transform) (BaseDamage :type Float%20%28single-precision%29))
  (bind _returnvalue (Game|SpawnActorfromClass "/Game/Characters/Projectiles/BP_Projectile_ThunderBall.BP_Projectile_ThunderBall_C" SpawnTransform "Undefined" (Components|GetOwner) 2.5e+03 0.0 0 false 0))
  (EventDispatchers|AssignOnProjectileImpact _returnvalue (delegate Custom|CustomEvent_1))
  (Collision|IgnoreActorwhenMoving (Variables|/Game/Characters/Projectiles/BP_Projectile_Base.BP_Projectile_Base_C|GetBoxCollision _returnvalue) (Components|GetOwner) true))

(event Custom|CustomEvent_1
  (params (OtherActor :type Actor%20Object%20Reference) (Hit :type Hit%20Result%20Structure))
  (bind _returnvalue (Components|GetOwner))
  (Utilities|Casting|CastToBP_ThirdPersonCharacter OtherActor)
  (Game|Damage|ApplyDamage OtherActor (stale Custom|ThunderSpell BaseDamage) (AI|GetAIController _returnvalue) (stale Custom|ThunderSpell _returnvalue))
  (Class|AISenseDamage|ReportDamageEvent OtherActor _returnvalue (stale Custom|ThunderSpell BaseDamage) (Transformation|GetActorLocation _returnvalue) "0, 0, 0" "None")
  (Camera|PlayWorldCameraShake "/Game/Enemies/AI/BP_HitShake.BP_HitShake_C" (.Location (Collision|BreakHitResult Hit)) 0.0 2e+03)
  (Default|CallOnAttackEnded))

(event Custom|FrenziedFire
  (params (SpawnTransform :type Transform) (BaseDamage :type Float%20%28single-precision%29))
  (bind _returnvalue (Game|SpawnActorfromClass "/Game/Characters/Projectiles/BP_Projectile_FrenziedFire.BP_Projectile_FrenziedFire_C" SpawnTransform "Undefined" (Components|GetOwner) 5e+02 0.0 (Game|Player|GetPlayerPawn 0) true 0))
  (EventDispatchers|AssignOnProjectileImpact _returnvalue (delegate Custom|CustomEvent_2))
  (Collision|IgnoreActorwhenMoving (Variables|/Game/Characters/Projectiles/BP_Projectile_Base.BP_Projectile_Base_C|GetBoxCollision _returnvalue) (Components|GetOwner) true))

(event EventBeginPlay)

(event EventTick
  (params (DeltaSeconds :type Float%20%28single-precision%29)))