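; BP_Patroller_Melee is a melee patroller enemy Blueprint that supplies the Attack behavior.
; Attack picks a random montage from Attacks and plays it on the mesh at the rate stored at the same index in the parallel AttackSpeeds array.
; Both completion and interruption of the montage broadcast OnAttackEnd, signaling that the attack is over.
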(event EventBeginPlay
  (|CallParentFunction) ; This node is disabled and will not be called.\nDrag off pins to build functionality.
)

(event EventAttack
  (bind _attacks (Variables|Default|GetAttacks))
  (bind _output_get (Variables|Default|Setindex (Math|Random|RandomInteger (Utilities|Array|Length _attacks))))
  (bind _output_get_2 (Variables|Default|SetAttackSpeed (Utilities|Array|Get(acopy) (Variables|Default|GetAttackSpeeds) _output_get)))
  (Animation|Montage|PlayMontage (Variables|Character|GetMesh) (Utilities|Array|Get(acopy) _attacks _output_get) _output_get_2
    (:OnCompleted
      _)
    (:OnInterrupted
      _))
  (Default|CallOnAttackEnd))

(event EventTick
  (params (DeltaSeconds :type Float%20%28single-precision%29))
  (|CallParentFunction DeltaSeconds) ; This node is disabled and will not be called.\nDrag off pins to build functionality.
)

(event Collision|EventActorBeginOverlap
  (params (OtherActor :type Actor%20Object%20Reference)))

(fn ConstructionScript
  (|CallParentFunction))