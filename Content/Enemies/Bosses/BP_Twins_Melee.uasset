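; Melee enemy Blueprint for the Twins boss, with its own health bar and ideal attack and defend ranges for the AI.
; Attack plays a random montage at its paired speed and signals attack end on completion or interruption.
; Damage is nearly negated except during root-motion montages, when it is boosted and spawns a player-oriented particle effect.
; Death sets the AI to dead, strips health bar and capsule, and ragdolls scrap with damage-scaled force.
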(event Custom|Update%20Damage%20Multiplication
  (bind _returnvalue (Game|GetPlayerCharacter 0))
  (bind _self self)
  (bind _returnvalue_2 (Transformation|GetActorLocation _returnvalue))
  (bind _returnvalue_3 (Transformation|GetActorLocation _self))
  (bind _returnvalue_4 (Math|Rotator|FindLookatRotation _returnvalue_3 _returnvalue_2))
  (if (Class|Character|IsPlayingNetworkedRootMotionMontage)
    (Variables|Default|SetDamage%20Multiplier 1.25)
    (Effects|SpawnEmitterAttached "/Game/Characters/P_Revenant_Obliterate_Firing_Local.P_Revenant_Obliterate_Firing_Local" (Variables|Default|GetCapsuleComponent) "None" "0, 0, 0" (Math|Rotator|MakeRotator (.roll _returnvalue_4) (.pitch _returnvalue_4) (+ (.yaw _returnvalue_4) 9e+01)) "1.000000,1.000000,1.000000" "SnapToTargetIncludingScale" false)
    (else
      (Variables|Default|SetDamage%20Multiplier 0.01))))

(event EventBeginPlay
  (|CallParentFunction) ; This node is disabled and will not be called.\nDrag off pins to build functionality.
)

(event EventAttack
  (bind _attacks (Variables|Default|GetAttacks))
  (bind _output_get (Variables|Default|Setindex (Math|Random|RandomInteger (Utilities|Array|Length _attacks))))
  (bind _output_get_2 (Variables|Default|SetAttackSpeed (Utilities|Array|Get(acopy) (Variables|Default|GetAttackSpeeds) _output_get)))
  (Animation|Montage|PlayMontage (Variables|Character|GetMesh) (Utilities|Array|Get(acopy) _attacks _output_get) _output_get_2
    (:OnCompleted
      _)
    (:OnInterrupted
      _))
  (Default|CallOnAttackEnd))

(event EventTick
  (params (DeltaSeconds :type Float%20%28single-precision%29)))

(event Collision|EventActorBeginOverlap
  (params (OtherActor :type Actor%20Object%20Reference)))

(event Game|Damage|EventAnyDamage
  (params (Damage :type Float%20%28single-precision%29) (DamageType :type Damage%20Type%20Object%20Reference) (InstigatedBy :type Controller%20Object%20Reference) (DamageCauser :type Actor%20Object%20Reference))
  (bind _damage_multiplier (Variables|Default|GetDamage%20Multiplier))
  (bind _bp_healthbar (Variables|Default|GetBP_HealthBar))
  (bind _returnvalue (* Damage _damage_multiplier))
  (CallFunction|UpdateDamageMultiplication)
  (if (not (Variables|Default|GetisDead))
    (Default|TakeDamage (Variables|Default|GetBP_HealthBar) _returnvalue)
    (Class|AISenseDamage|ReportDamageEvent self DamageCauser _returnvalue (Transformation|GetActorLocation DamageCauser) "0, 0, 0" "None")
    (if (<= (Variables|/Game/Blueprints/BP_HealthBar.BP_HealthBar_C|GetHealth (Variables|Default|GetBP_HealthBar)) 0.0)
      (Components|Movement|StopMovementImmediately (Variables|Character|GetCharacterMovement))
      (bind _asaic_enemy_base (Utilities|Casting|CastToAIC_Enemy_Base (AI|GetAIController self)))
      (Default|SetStateasDead _asaic_enemy_base)
      (Variables|Default|SetisDead true)
      (Default|DisableHealthBar _bp_healthbar)
      (Components|DestroyComponent _bp_healthbar)
      (Components|DestroyComponent (Variables|Default|GetCapsuleComponent))
      (Default|RagdollScrap (Variables|Default|GetdeathScrap) self (Variables|Character|GetMesh) "None" (* _returnvalue 1.3e+05)))))

(fn ConstructionScript
  (|CallParentFunction)
  (Variables|/Game/Blueprints/BP_HealthBar.BP_HealthBar_C|SetMaxHealth (Variables|Default|GetBP_HealthBar) 1e+02))

(fn GetIdealRange
  (return 1.7e+02 3.5e+02))