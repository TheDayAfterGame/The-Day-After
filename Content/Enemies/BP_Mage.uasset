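; BP_Mage is a ranged enemy character that attacks with a fireball spell.
; Attack plays the fireball montage and signals attack end when it completes or is interrupted.
; On the montage notify, it checks the AI controller's attack target, then has BPCAttacks cast MagicSpell from the left hand along the actor's facing rather than toward the target.
; It also supplies its own movement speeds and long attack and defend ranges.
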(event EventBeginPlay
  (|CallParentFunction) ; This node is disabled and will not be called.\nDrag off pins to build functionality.
)

(event Collision|EventActorBeginOverlap
  (params (OtherActor :type Actor%20Object%20Reference)))

(event EventTick
  (params (DeltaSeconds :type Float%20%28single-precision%29)))

(event EventAttack
  (bind _notifyname (Animation|Montage|PlayMontage (Variables|Character|GetMesh) "/Game/Characters/EnemyMage/Animations/Montage_Mage_Fireball.Montage_Mage_Fireball")
    (:OnCompleted
      (Default|CallOnAttackEnd :!label _label))
    (:OnInterrupted
      (goto _label))
    (:OnNotifyBegin
      (switch name _notifyname
        (:Fire
          (bind _asaic_enemy_base (Utilities|Casting|CastToAIC_Enemy_Base (AI|GetAIController self)))
          (bind _attacktarget (Variables|/Game/Enemies/AI/AIC_Enemy_Base.AIC_Enemy_Base_C|GetAttackTarget _asaic_enemy_base)
            (:then
              (Default|MagicSpell (Variables|Default|GetBPC_Attacks) (Math|Transform|MakeTransform (Transformation|GetSocketLocation (Variables|Character|GetMesh) "LeftHand") (Transformation|GetActorRotation self) "1.000000,1.000000,1.000000") 2e+01))
            (:else)))))))

(fn ConstructionScript
  (|CallParentFunction))

(fn SetMovementSpeed
  (params (Speed :type E_MovementSpeed%20Enum :default "NewEnumerator0"))
  (return (Utilities|Select :Index Speed :NewEnumerator0 0.0 :NewEnumerator1 1.5e+02 :NewEnumerator2 2.5e+02 :NewEnumerator3 4e+02 :NewEnumerator4 0.0)))

(fn GetIdealRange
  (return 7e+02 9e+02))