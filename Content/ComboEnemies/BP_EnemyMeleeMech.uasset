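; BP_EnemyMeleeMech is a melee enemy that attacks the player with random montages.
; On BeginPlay it attaches a BP_Sword with hidden mesh to its fist socket.
; Attack rolls speed, socket index and montage independently, then signals attack end on completion or interruption.
; HitDetect sphere-traces at the indexed socket, applying damage, blood, camera shake and sound, with a flag blocking repeat hits until a trace misses.
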(event EventBeginPlay
  (bind _returnvalue (Game|SpawnActorfromClass "/Game/Weapons/BP_Sword.BP_Sword_C" (Transformation|GetActorTransform) "Undefined" 0 0))
  (Rendering|SetVisibility (Variables|/Game/Weapons/BP_Sword.BP_Sword_C|GetSwordMesh _returnvalue) false false)
  (bind _output_get (Variables|Default|SetSwordActor _returnvalue))
  (Transformation|AttachComponentToComponent _output_get (Variables|Character|GetMesh) "FistSocket" "SnapToTarget" "SnapToTarget" "SnapToTarget" true)
  (Variables|Default|SetisWieldingSword true))

(event EventAttack
  (bind _attacks (Variables|Default|GetAttacks))
  (bind _returnvalue (Utilities|Array|Length _attacks))
  (bind _returnvalue_2 (Math|Random|RandomInteger _returnvalue))
  (bind _output_get (Variables|Default|SetAttackSpeed (Utilities|Array|Get(acopy) (Variables|Default|GetAttackSpeeds) _returnvalue_2)))
  (Variables|Default|SetAttackIndex _returnvalue_2)
  (Animation|Montage|PlayMontage (Variables|Character|GetMesh) (Utilities|Array|Get(acopy) _attacks _returnvalue_2) _output_get
    (:OnCompleted
      _)
    (:OnInterrupted
      _))
  (Default|CallOnAttackEnd))

(fn ConstructionScript
  (|CallParentFunction))

(fn HitDetect
  (bind _mesh (Variables|Character|GetMesh))
  (bind _attackindex (Variables|Default|GetAttackIndex))
  (bind _attackattachnames (Variables|Default|GetAttackAttachNames))
  (bind _output (Utilities|Array|Get(acopy) _attackattachnames _attackindex))
  (bind _returnvalue (Transformation|GetSocketLocation _mesh _output))
  (Development|PrintString (Utilities|String|ToString(Name) _output))
  (bind (_outhit _returnvalue_2) (Collision|SphereTraceForObjects _returnvalue _returnvalue 1e+01 (Utilities|Array|MakeArray "ObjectTypeQuery3") false 0 "ForDuration"))
  (if _returnvalue_2
    (if (not (Variables|Default|GetwasJustHit))
      (bind _asbp_third_person_character (Utilities|Casting|CastToBP_ThirdPersonCharacter (.HitActor (Collision|BreakHitResult _outhit))))
      (Game|Damage|ApplyDamage _asbp_third_person_character 1e+01 0 self)
      (Effects|SpawnEmitteratLocation "/Game/Realistic_Starter_VFX_Pack_Vol2/Particles/Blood/P_Blood_Splat_Cone.P_Blood_Splat_Cone" (.Location (Collision|BreakHitResult _outhit)) (Math|Rotator|MakeRotfromXY (.Normal (Collision|BreakHitResult _outhit)) (.Normal (Collision|BreakHitResult _outhit))) "1.000000,1.000000,1.000000" true "AutoRelease")
      (Camera|PlayWorldCameraShake "/Game/Enemies/AI/BP_HitShake.BP_HitShake_C" (.Location (Collision|BreakHitResult _outhit)) 0.0 2e+03)
      (Audio|PlaySoundatLocation "/Game/Characters/Patrolller/MetaSounds/MT_HitPlayer.MT_HitPlayer" (.Location (Collision|BreakHitResult _outhit)) "0, 0, 0" 1.0 1.0 0.0 0 0 0 0)
      (Variables|Default|SetwasJustHit true))
    (else
      (Variables|Default|SetwasJustHit false))))