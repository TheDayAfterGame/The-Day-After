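; Base sword enemy character with a health bar, patrol route and speed presets, paired with AIC_Enemy_Base.
; Investigate, wield and sheath montages fire end dispatchers, while separate events spawn or destroy the socketed sword.
; HitDetect sphere-traces along the blade to damage the player once per contact, with effects.
; Damage is reported to AI sensing; death ragdolls via DeathScrap; Attack is empty and its combo logic is disconnected.
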(event Custom|Wield%20Sword
  (Animation|Montage|PlayMontage (Variables|Character|GetMesh) 0
    (:OnCompleted
      _)
    (:OnInterrupted
      _))
  (Default|CallOnWieldEnd))

(event Custom|Remove%20Sword
  (Actor|DestroyActor (Variables|Default|GetSwordActor))
  (Variables|AI|SetisWieldingSword false))

(event Custom|Spawn%20Sword
  (bind _returnvalue (Game|SpawnActorfromClass "/Game/Weapons/BP_Sword.BP_Sword_C" (Transformation|GetActorTransform) "Undefined" 0 0))
  (bind _output_get (Variables|Default|SetSwordActor _returnvalue))
  (Transformation|AttachComponentToComponent _output_get (Variables|Character|GetMesh) "SwordSocket" "SnapToTarget" "SnapToTarget" "SnapToTarget" true)
  (Variables|AI|SetisWieldingSword true))

(event Custom|Sheath%20Sword
  (Animation|Montage|PlayMontage (Variables|Character|GetMesh) 0
    (:OnCompleted
      _)
    (:OnInterrupted
      _))
  (Default|CallOnSheathEnd))

(event Custom|Investigate
  (Animation|Montage|PlayMontage (Variables|Character|GetMesh) 0 0.5
    (:OnCompleted
      _)
    (:OnInterrupted
      _))
  (Default|CallOnInvestigateEnd))

(event EventBeginPlay
  (Default|UpdateHealthBar (Variables|Default|GetBP_HealthBar)))

(event Game|Damage|EventAnyDamage
  (params (Damage :type Float%20%28single-precision%29) (DamageType :type Damage%20Type%20Object%20Reference) (InstigatedBy :type Controller%20Object%20Reference) (DamageCauser :type Actor%20Object%20Reference))
  (bind _bp_healthbar (Variables|Default|GetBP_HealthBar))
  (if (not (Variables|Default|GetisDead))
    (Default|TakeDamage (Variables|Default|GetBP_HealthBar) Damage)
    (Class|AISenseDamage|ReportDamageEvent self DamageCauser Damage (Transformation|GetActorLocation DamageCauser) "0, 0, 0" "None")
    (if (<= (Variables|/Game/Blueprints/BP_HealthBar.BP_HealthBar_C|GetHealth (Variables|Default|GetBP_HealthBar)) 0.0)
      (Components|Movement|StopMovementImmediately (Variables|Character|GetCharacterMovement))
      (bind _asaic_enemy_base (Utilities|Casting|CastToAIC_Enemy_Base (AI|GetAIController self)))
      (Default|SetStateasDead _asaic_enemy_base)
      (Variables|Default|SetisDead true)
      (CallFunction|RemoveSword)
      (Components|DestroyComponent (Variables|Default|GetSword))
      (Default|DisableHealthBar _bp_healthbar)
      (Components|DestroyComponent _bp_healthbar)
      (Components|DestroyComponent (Variables|Collision|GetCapsuleComponent))
      (Default|RagdollScrap (Variables|Default|GetdeathScrap) self (Variables|Character|GetMesh) "None" (* Damage 1.3e+05)))))

(event EventAttack)

(event EventTick
  (params (DeltaSeconds :type Float%20%28single-precision%29)))

(fn ConstructionScript
  (CallFunction|RemoveSword))

(fn HitDetect
  (bind (_outhit _returnvalue) (Collision|SphereTraceForObjects (Transformation|GetSocketLocation (Variables|Character|GetMesh) "SwordSocket") (Transformation|GetWorldLocation (Variables|Default|GetArrow1)) 1e+01 (Utilities|Array|MakeArray "ObjectTypeQuery3") false 0 "ForDuration"))
  (if _returnvalue
    (if (not (Variables|AI|GetwasJustHit))
      (bind _asbp_third_person_character (Utilities|Casting|CastToBP_ThirdPersonCharacter (.HitActor (Collision|BreakHitResult _outhit))))
      (Game|Damage|ApplyDamage _asbp_third_person_character 1e+01 0 self)
      (Effects|SpawnEmitteratLocation "/Game/Realistic_Starter_VFX_Pack_Vol2/Particles/Blood/P_Blood_Splat_Cone.P_Blood_Splat_Cone" (.Location (Collision|BreakHitResult _outhit)) (Math|Rotator|MakeRotfromXY (.Normal (Collision|BreakHitResult _outhit)) (.Normal (Collision|BreakHitResult _outhit))) "1.000000,1.000000,1.000000" true "AutoRelease")
      (Camera|PlayWorldCameraShake "/Game/Enemies/AI/BP_HitShake.BP_HitShake_C" (.Location (Collision|BreakHitResult _outhit)) 0.0 2e+03)
      (Audio|PlaySoundatLocation 0 (.Location (Collision|BreakHitResult _outhit)) "0, 0, 0" 1.0 1.0 0.0 0 0 0 0)
      (Variables|AI|SetwasJustHit true))
    (else
      (Variables|AI|SetwasJustHit false))))

(fn GetIdealRange
  (return 0.0 0.0))

(fn GetPatrolRoute
  (return (Variables|AI|GetPatrolRoute)))

(fn SetMovementSpeed
  (params (Speed :type E_MovementSpeed%20Enum :default "NewEnumerator0"))
  (bind _returnvalue (Utilities|Select :Index Speed :NewEnumerator0 0.0 :NewEnumerator1 1e+02 :NewEnumerator2 3e+02 :NewEnumerator3 5e+02 :NewEnumerator4 0.0))
  (bind _output_get (Variables|/Script/Engine.CharacterMovementComponent|SetMaxWalkSpeed (Variables|Character|GetCharacterMovement) _returnvalue))
  (Variables|AI|SetisSprinting (== _returnvalue 5e+02))
  (return _output_get))